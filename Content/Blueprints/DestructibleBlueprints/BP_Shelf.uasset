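; BP_Shelf is a breakable factory shelf that shatters and collapses when it takes any damage.
; On AnyDamage it applies strong, full radius damage from the actor's origin to three Shelves1 destructible mesh pieces, fracturing them with an impulse.
; It then enables physics simulation on those pieces and two Shelves2 pieces, which receive no radius damage.
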(event `self.ReceiveAnyDamage`
  (params (Damage :type "Float (single-precision)") (DamageType :type "DamageType Object Reference") (InstigatedBy :type "Controller Object Reference") (DamageCauser :type "Actor Object Reference"))
  (`DestructibleComponent.ApplyRadiusDamage` (`self.FactoryLevel1Assets_model_shelves_1_polySurface2_DM`) 100.0 (`self.K2_GetActorLocation`) 10000.0 1000.0 true)
  (`DestructibleComponent.ApplyRadiusDamage` (`self.FactoryLevel1Assets_model_shelves_1_polySurface1_DM`) 100.0 (`self.K2_GetActorLocation`) 10000.0 1000.0 true)
  (`DestructibleComponent.ApplyRadiusDamage` (`self.FactoryLevel1Assets_model_shelves_1_polySurface3_DM`) 100.0 (`self.K2_GetActorLocation`) 10000.0 1000.0 true)
  (`PrimitiveComponent.SetSimulatePhysics` (`self.FactoryLevel1Assets_model_shelves_1_polySurface2_DM`) true)
  (`PrimitiveComponent.SetSimulatePhysics` (`self.FactoryLevel1Assets_model_shelves_1_polySurface1_DM`) true)
  (`PrimitiveComponent.SetSimulatePhysics` (`self.FactoryLevel1Assets_model_shelves_1_polySurface3_DM`) true)
  (`PrimitiveComponent.SetSimulatePhysics` (`self.FactoryLevel1Assets_model_shelves_2_polySurface5_DM`) true)
  (`PrimitiveComponent.SetSimulatePhysics` (`self.FactoryLevel1Assets_model_shelves_2_polySurface6_DM`) true))

(fn `UserConstructionScript`)