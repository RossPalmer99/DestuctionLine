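; Throwable barrel that explodes when damaged if its item colour is red, using a destructible mesh instead of the static one.
; Damage from non-barrel causers starts a brief fire, then fractures it, fires a radial impulse, triggers nearby characters' held items, damages overlapping actors and destroys itself.
; Fast thrown impacts damage barrel and target, with a DoOnce gating the thrower's points for character hits.
; Explosion decal spawning is unconnected.
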(event `self.ReceiveBeginPlay`
  (bind (_iteminfo_isproduct _iteminfo_isweapon1h _iteminfo_isweapon2h _iteminfo_isstacktruck _iteminfo_isfireextinguisher _iteminfo_isaccessory _iteminfo_ispowerup _iteminfo_isalarmclock _iteminfo_isbarrel _iteminfo_damage _iteminfo_weaponpower _iteminfo_weaponchip _iteminfo_colour) (break `/Game/Blueprints/Items/Data/Struct_ItemInfo` (`self.ItemInfo`)))
  ;[1 1 1] Begin Play - set barrel colour
  (`parent.ReceiveBeginPlay`)
  (if (== _iteminfo_colour "Red")
    (`SceneComponent.SetVisibility` (`self.StaticMesh`) false false)
    (`SceneComponent.SetVisibility` (`self.Destructible`) true false)
    (else
      (`SceneComponent.SetVisibility` (`self.StaticMesh`) true false)
      (`SceneComponent.SetVisibility` (`self.Destructible`) false false))))

(event `self.ReceiveAnyDamage`
  (params (Damage :type "Float (single-precision)") (DamageType :type "DamageType Object Reference") (InstigatedBy :type "Controller Object Reference") (DamageCauser :type "Actor Object Reference"))
  (bind (_iteminfo_isproduct _iteminfo_isweapon1h _iteminfo_isweapon2h _iteminfo_isstacktruck _iteminfo_isfireextinguisher _iteminfo_isaccessory _iteminfo_ispowerup _iteminfo_isalarmclock _iteminfo_isbarrel _iteminfo_damage _iteminfo_weaponpower _iteminfo_weaponchip _iteminfo_colour) (break `/Game/Blueprints/Items/Data/Struct_ItemInfo` (`self.ItemInfo`)))
  ;[1 1 1] Event Damage
  (if (!= (`GameplayStatics.GetObjectClass` DamageCauser) (`GameplayStatics.GetObjectClass` self))
    (if (== _iteminfo_colour "Red")
      (`ActorComponent.Activate` (`self.Fire`) false)
      (`KismetSystemLibrary.Delay` 2.0)
      (`ActorComponent.Deactivate` (`self.Fire`))
      (`DestructibleComponent.ApplyRadiusDamage` (`self.Destructible`) 100.0 (`self.K2_GetActorLocation`) 0.0 15000.0 true)
      (bind _playerref (`self.PlayerRef`)
        (:`then`
          (bind _helditem (`/Game/Blueprints/Characters/Golem/0_Base.HeldItem` _playerref)
            (:`then`
              (message `/Game/Data/Interact_Interface.Interact` _helditem _playerref))
            (:`else`
              _)))
        (:`else`
          _))
      (`self.Explosion`)
      (`KismetSystemLibrary.Delay` 1e-05)
      (for _array_element (`PrimitiveComponent.GetOverlappingActors` (`self.DetectionSphere`) null)
        (bind _as0_base (cast `/Game/Blueprints/Characters/Golem/0_Base` _array_element)
          (:`then`
            (bind _helditem_2 (`/Game/Blueprints/Characters/Golem/0_Base.HeldItem` _as0_base)
              (:`then`
                (message `/Game/Data/Interact_Interface.Interact` _helditem_2 _as0_base))
              (:`else`
                _)))
          (:`CastFailed`
            _))
        (`GameplayStatics.ApplyDamage` _array_element 10.0 null self)
        (`GameplayStatics.SpawnForceFeedbackAttached` "/Game/Blueprints/Characters/Golem/Vibration_Pack/FF_FLT.FF_FLT" (`self.StaticMesh`) "None" (0.0 0.0 0.0) (struct) "SnapToTarget" false false 1.5 0.0 (`self.Falloff`)))
      (`self.SetActorEnableCollision` false)
      (`PrimitiveComponent.SetCollisionEnabled` (`self.Destructible`) "QueryAndPhysics")
      (`KismetSystemLibrary.Delay` 5.0)
      (`self.K2_DestroyActor`))))

(event `ResetDoOnce`
  ;[1 1 1] Throw
  (goto _label :!via `Reset`))

(event `Throw`
  (params (PlayerThrowing :type "/Game/Blueprints/Characters/Golem/0_Base Object Reference"))
  ;[1 1 1] Throw
  (bind _output_get (set `self.HasBeenThrown` true)))

(event `self.ReceiveHit`
  (params (MyComp :type "PrimitiveComponent Object Reference") (Other :type "Actor Object Reference") (OtherComp :type "PrimitiveComponent Object Reference") (bSelfMoved :type Boolean) (HitLocation :type "Vector Structure") (HitNormal :type "Vector Structure") (NormalImpulse :type "Vector Structure") (Hit :type "HitResult Structure (by ref)"))
  ;[1 1 1] Throw
  (if (and (stale `Throw` _output_get) (!= (stale `Throw` PlayerThrowing) Other))
    (if (!= (`self.GetVelocity` self) (0.0 0.0 0.0) :`ErrorTolerance` 200.0)
      (`GameplayStatics.ApplyDamage` self 10.0 null (stale `Throw` PlayerThrowing))
      (`GameplayStatics.ApplyDamage` Other 10.0 null (stale `Throw` PlayerThrowing))
      (if (== (`GameplayStatics.GetObjectClass` Other) "/Game/Blueprints/Characters/Golem/0_Base.0_Base_C")
        (`/Engine/EditorBlueprintResources/StandardMacros.DoOnce` false :!label _label
          (:`Completed`
            (`self.GivePoints` (`KismetMathLibrary.FTrunc` (* 10 (`/Game/Blueprints/Characters/Golem/0_Base.PointMultiplier` (stale `Throw` PlayerThrowing)))) (stale `Throw` PlayerThrowing))
            (message `/Game/Data/Interact_Interface.UpdateScore` (`/Game/Blueprints/Characters/Golem/0_Base.Scoreboard` (stale `Throw` PlayerThrowing)))
            (`self.PlaySound`)
            (`PlayerController.K2_ClientPlayForceFeedback` (`GameplayStatics.GetPlayerController` (`/Game/Blueprints/Characters/Golem/0_Base.Index` (stale `Throw` PlayerThrowing))) (`/Game/Blueprints/Characters/Golem/0_Base.FF_2hHit` (stale `Throw` PlayerThrowing)) "None" false false false))))
      (else
        (set `self.HasBeenThrown` false)))))

(fn `Explosion`
  (`RadialForceComponent.FireImpulse` (`self.RadialForce`)))

(fn `UserConstructionScript`
  (`parent.UserConstructionScript`))