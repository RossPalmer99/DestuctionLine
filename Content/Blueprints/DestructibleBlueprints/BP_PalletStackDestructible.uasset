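; BP_PalletStackDestructible is a pallet stack that breaks apart when it takes any damage.
; On damage, it applies radius damage with an impulse from the actor's location to five destructible components and turns on their physics.
; It then disables collision on the Box component.
; A breaking sound node exists but never runs, and the trailing DoOnce drives nothing, so the damage response is not gated.
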(event `self.ReceiveAnyDamage`
  (params (Damage :type "Float (single-precision)") (DamageType :type "DamageType Object Reference") (InstigatedBy :type "Controller Object Reference") (DamageCauser :type "Actor Object Reference"))
  (`DestructibleComponent.ApplyRadiusDamage` (`self.Destructible`) 1.0 (`self.K2_GetActorLocation`) 1000.0 1000.0 true)
  (`DestructibleComponent.ApplyRadiusDamage` (`self.Destructible1`) 1.0 (`self.K2_GetActorLocation`) 1000.0 1000.0 true)
  (`DestructibleComponent.ApplyRadiusDamage` (`self.Destructible2`) 1.0 (`self.K2_GetActorLocation`) 1000.0 1000.0 true)
  (`DestructibleComponent.ApplyRadiusDamage` (`self.Destructible3`) 1.0 (`self.K2_GetActorLocation`) 1000.0 1000.0 true)
  (`DestructibleComponent.ApplyRadiusDamage` (`self.Destructible4`) 1.0 (`self.K2_GetActorLocation`) 1000.0 1000.0 true)
  (`PrimitiveComponent.SetSimulatePhysics` (`self.Destructible`) true)
  (`PrimitiveComponent.SetSimulatePhysics` (`self.Destructible1`) true)
  (`PrimitiveComponent.SetSimulatePhysics` (`self.Destructible2`) true)
  (`PrimitiveComponent.SetSimulatePhysics` (`self.Destructible3`) true)
  (`PrimitiveComponent.SetSimulatePhysics` (`self.Destructible4`) true)
  (`PrimitiveComponent.SetCollisionEnabled` (`self.Box`) "NoCollision")
  (`/Engine/EditorBlueprintResources/StandardMacros.DoOnce` false))

(fn `UserConstructionScript`)