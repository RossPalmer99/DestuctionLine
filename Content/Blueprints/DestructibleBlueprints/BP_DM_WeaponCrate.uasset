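; Destructible weapon crate that breaks on any damage, drops a random weapon and awards points to the player who damaged it.
; Damage applies radius damage and physics to the destructible mesh while turning off the static mesh's physics and collision.
; After a short delay, a DoOnce spawns a weapon from a random numbered WeaponSpawnChance table row.
; It then adds multiplier-scaled round points to the damaging 0_Base's PlayerInfo and updates its scoreboard message.
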(event `self.ReceiveAnyDamage`
  (params (Damage :type "Float (single-precision)") (DamageType :type "DamageType Object Reference") (InstigatedBy :type "Controller Object Reference") (DamageCauser :type "Actor Object Reference"))
  (bind _staticmesh (`self.StaticMesh`))
  (`DestructibleComponent.ApplyRadiusDamage` (`self.MoreAssets_model_item_crate_DM`) 100.0 (`self.K2_GetActorLocation`) 0.0 100.0 true)
  (`PrimitiveComponent.SetSimulatePhysics` (`self.MoreAssets_model_item_crate_DM`) true)
  (`PrimitiveComponent.SetSimulatePhysics` _staticmesh false)
  (`PrimitiveComponent.SetCollisionEnabled` _staticmesh "NoCollision")
  (`KismetSystemLibrary.Delay` 0.2)
  (`/Engine/EditorBlueprintResources/StandardMacros.DoOnce` false
    (:`Completed`
      (`self.SpawnWeapon`)
      (bind _as0_base (cast `/Game/Blueprints/Characters/Golem/0_Base` DamageCauser))
      (bind (_playerinfo_playername _playerinfo_rank _playerinfo_items_crafted _playerinfo_products_shipped _playerinfo_tasks_completed _playerinfo_players_knocked_out _playerinfo_players_knocked_out_unarmed _playerinfo_players_knocked_out_1h _playerinfo_players_knocked_out_2h _playerinfo_players_knocked_out_sp _playerinfo_players_knocked_out_ra _playerinfo_times_taunted _playerinfo_pointsround _playerinfo_outfit) (break `/Game/Blueprints/Characters/Golem/Struct_PlayerInfo` (`/Game/Blueprints/Characters/Golem/0_Base.PlayerInfo` _as0_base)))
      (set `/Game/Blueprints/Characters/Golem/0_Base.PlayerInfo` (make `/Game/Blueprints/Characters/Golem/Struct_PlayerInfo` _playerinfo_playername _playerinfo_rank _playerinfo_items_crafted _playerinfo_products_shipped _playerinfo_tasks_completed _playerinfo_players_knocked_out _playerinfo_players_knocked_out_unarmed _playerinfo_players_knocked_out_1h _playerinfo_players_knocked_out_2h _playerinfo_players_knocked_out_sp _playerinfo_players_knocked_out_ra _playerinfo_times_taunted (+ _playerinfo_pointsround (`KismetMathLibrary.FTrunc` (* 2 (`/Game/Blueprints/Characters/Golem/0_Base.PointMultiplier` _as0_base)))) _playerinfo_outfit) _as0_base)
      (message `/Game/Data/Interact_Interface.UpdateScore` (`/Game/Blueprints/Characters/Golem/0_Base.Scoreboard` _as0_base)))))

(fn `SpawnWeapon`
  (bind _returnvalue (`|GetDataTableRow` "/Game/Blueprints/Items/Data/WeaponSpawnChance.WeaponSpawnChance" (`KismetStringLibrary.Conv_StringToName` (`KismetStringLibrary.Conv_IntToString` (`KismetMathLibrary.RandomIntegerInRange` 0 499))))
    (:`then`
      (`|SpawnActorFromClass` (`.FactoryWeapons_24_7DEF36094858E9FD296E7C88695CBD73` (break `/Game/Blueprints/Items/Data/Struct_WeaponArray` _returnvalue)) (`KismetMathLibrary.MakeTransform` (`self.K2_GetActorLocation`) (`self.K2_GetActorRotation`)) "Undefined" "OverrideRootScale" null null))))

(fn `UserConstructionScript`)