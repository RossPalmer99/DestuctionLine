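; Behavior Tree task that picks a point away from the nearest 0_Base actor, treated as a player, for the controlled AI pawn.
; On execute it gathers every such actor's distance and location into parallel arrays, filled with AddUnique, and selects the closest.
; It offsets the pawn's location horizontally along the look-at direction from that actor, writes the result to a Blackboard vector, clears both arrays and finishes successfully.
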(event `self.ReceiveExecuteAI`
  (params (OwnerController :type "AIController Object Reference") (ControlledPawn :type "Pawn Object Reference"))
  (set `self.AIPawn` ControlledPawn)
  (set `self.MyCurrentLocation` (`Actor.K2_GetActorLocation` (`self.AIPawn`)))
  (bind _outactors (`GameplayStatics.GetAllActorsOfClass` "/Game/Blueprints/Characters/Golem/0_Base.0_Base_C"))
  (for _array_element _outactors
    (bind _returnvalue (`Actor.K2_GetActorLocation` _array_element))
    (`KismetArrayLibrary.Array_AddUnique` (`self.DistanceToPlayers`) (`KismetMathLibrary.Vector_Distance` (`self.MyCurrentLocation`) _returnvalue))
    (`KismetArrayLibrary.Array_AddUnique` (`self.AllPlayerLocations`) _returnvalue))
  (`BTFunctionLibrary.SetBlackboardValueAsVector` (`self.Vector`) (+ (`self.MyCurrentLocation`) (* (`KismetMathLibrary.GetForwardVector` (`KismetMathLibrary.FindLookAtRotation` (`|GetArrayItem` (`self.AllPlayerLocations`) (`KismetMathLibrary.MinOfFloatArray` (`self.DistanceToPlayers`))) (`self.MyCurrentLocation`))) (500.0 500.0 0.0))))
  (`KismetArrayLibrary.Array_Clear` (`self.DistanceToPlayers`))
  (`KismetArrayLibrary.Array_Clear` (`self.AllPlayerLocations`))
  (`self.FinishExecute` true))