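; BP_CarrotAI is the AI controller for the carrot AI, driven by the BT_CarrotAI behavior tree.
; It starts the tree on BeginPlay, and its AIPerception component feeds the blackboard.
; On each perception update for a 0_Base actor, it writes that actor as Player, itself as SelfActor, and the sensed result as CanSeePlayer.
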(event `self.ReceiveBeginPlay`
  (`self.RunBehaviorTree` "/Game/Blueprints/AI/CarrotAI/BT_CarrotAI.BT_CarrotAI"))

(event `self.AIPerception.OnTargetPerceptionUpdated`
  (params (Actor :type "Actor Object Reference") (Stimulus :type "AIStimulus Structure"))
  (bind _as0_base (cast `/Game/Blueprints/Characters/Golem/0_Base` Actor))
  (`BlackboardComponent.SetValueAsObject` (`AIBlueprintHelperLibrary.GetBlackboard` null) "Player" _as0_base)
  (`BlackboardComponent.SetValueAsObject` (`AIBlueprintHelperLibrary.GetBlackboard` null) "SelfActor" self)
  (`BlackboardComponent.SetValueAsBool` (`AIBlueprintHelperLibrary.GetBlackboard` null) "CanSeePlayer" (`.bSuccessfullySensed` (break `AIStimulus` Stimulus))))

(fn `UserConstructionScript`)