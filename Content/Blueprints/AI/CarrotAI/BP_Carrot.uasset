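; BP_Carrot is an AI carrot character that hops in place on a repeating timer.
; On BeginPlay it starts a looping timer that calls Jump every second.
; It also snaps its static mesh to the skeletal mesh's HeadLocation socket, keeping world scale, and rotates it to fit.
; A forward movement input node exists but is unconnected, and Tick is empty.
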(event `self.ReceiveBeginPlay`
  (`KismetSystemLibrary.K2_SetTimerDelegate` (delegate `Jumping`) 1.0 true)
  (`SceneComponent.K2_AttachToComponent` (`self.StaticMesh`) (`self.Mesh`) "HeadLocation" "SnapToTarget" "SnapToTarget" "KeepWorld" true)
  (`SceneComponent.K2_AddRelativeRotation` (`self.StaticMesh`) (struct :`Roll` -90.0) false false))

(event `Jumping`
  (`self.Jump`))

(event `self.ReceiveTick`
  (params (DeltaSeconds :type "Float (single-precision)")))

(fn `UserConstructionScript`)