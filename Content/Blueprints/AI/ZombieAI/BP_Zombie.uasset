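; Zombie enemy that punches in melee, takes damage and bursts into a random limb pickup or prop on death.
; MeleeAttack plays a montage whose notify runs Punch, damaging other actors overlapping FistCollision.
; A DoOnce gates incoming hits until the hit montage ends, with health reduced on its notify.
; The damage causer receives points and KO messages; death spawns a particle burst before destroying the zombie.
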(event `/Game/Blueprints/AI/ZombieAI/BP_CombatInterface.MeleeAttack`
  (`|PlayMontage` (`self.Mesh`) "/Game/Blueprints/Characters/Golem/Anims/OneHanded/Golem_WeaponAttack_1h_Montage.Golem_WeaponAttack_1h_Montage"
    (:`OnNotifyBegin`
      (`self.Punch`))))

(event `Reset`
  (goto _label :!via `Reset`))

(event `self.ReceiveAnyDamage`
  (params (Damage :type "Float (single-precision)") (DamageType :type "DamageType Object Reference") (InstigatedBy :type "Controller Object Reference") (DamageCauser :type "Actor Object Reference"))
  (`KismetSystemLibrary.PrintString` (`KismetStringLibrary.Conv_IntToString` (`self.Health`)))
  (if (> (`self.Health`) 0)
    (`/Engine/EditorBlueprintResources/StandardMacros.DoOnce` false :!label _label
      (:`Completed`
        (message `/Game/Data/Interact_Interface.Points` DamageCauser)
        (`|PlayMontage` (`self.Mesh`) "/Game/Blueprints/Characters/Golem/Anims/Golem_Hit_Montage.Golem_Hit_Montage"
          (:`OnCompleted`
            (`self.Reset` :!label _label_2))
          (:`OnInterrupted`
            (goto _label_2))
          (:`OnNotifyBegin`
            (set `self.Health` (- (`self.Health`) (`KismetMathLibrary.FTrunc` Damage)))
            (if (<= (`self.Health`) 0)
              (if (!= DamageCauser self)
                (message `/Game/Data/Interact_Interface.KOPoints` DamageCauser)
                (`self.Reset`)
                (`GameplayStatics.SpawnEmitterAtLocation` "/Game/Blueprints/Particles/PFX_CloudBurst.PFX_CloudBurst" (`self.K2_GetActorLocation`) (struct) (0.5 0.5 0.5))
                (`|SpawnActorFromClass` (`|GetArrayItem` (`self.LimbToSpawn`) (`KismetMathLibrary.RandomIntegerInRange` 0 (- (`KismetArrayLibrary.Array_Length` (`self.LimbToSpawn`)) 1))) (`KismetMathLibrary.MakeTransform` (`self.K2_GetActorLocation`)) "Undefined" "OverrideRootScale" null null)
                (`self.K2_DestroyActor`)))))))))

(fn `Punch`
  (for _array_element (`PrimitiveComponent.GetOverlappingActors` (`self.FistCollision`) "/Game/Blueprints/Characters/Golem/0_Base.0_Base_C")
    (if (!= _array_element self)
      (`GameplayStatics.ApplyDamage` _array_element 1.0 null self))))

(fn `UserConstructionScript`)