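; BP_Refrigerator is an environment prop whose hinged door swings open on interaction and closes when the actor takes damage.
; Interact plays the DoorAnimation timeline to drive the Hinge's yaw, and AnyDamage reverses it.
; Each timeline update also uses the Open flag to set both doors to ignore the Visibility channel while open and block it while closing.
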(event `/Game/Data/Interact_Interface.Interact`
  (params (Player :type "/Game/Blueprints/Characters/Golem/0_Base Object Reference"))
  (set `self.Open` true)
  (bind (_direction _rotation) (`Timeline|DoorAnimation` :!label _label)
    (:`Update`
      (`SceneComponent.K2_SetRelativeRotation` (`self.Hinge`) (`KismetMathLibrary.MakeRotator` 0.0 0.0 (* _rotation -140.0)) false false)
      (if (`self.Open`)
        (`PrimitiveComponent.SetCollisionResponseToChannel` (`self.Top_Door`) "ECC_Visibility" "ECR_Ignore")
        (`PrimitiveComponent.SetCollisionResponseToChannel` (`self.Bottom_Door`) "ECC_Visibility" "ECR_Ignore")
        (else
          (`PrimitiveComponent.SetCollisionResponseToChannel` (`self.Top_Door`) "ECC_Visibility" "ECR_Block")
          (`PrimitiveComponent.SetCollisionResponseToChannel` (`self.Bottom_Door`) "ECC_Visibility" "ECR_Block"))))))

(event `self.ReceiveAnyDamage`
  (params (Damage :type "Float (single-precision)") (DamageType :type "DamageType Object Reference") (InstigatedBy :type "Controller Object Reference") (DamageCauser :type "Actor Object Reference"))
  (set `self.Open` false)
  (goto _label :!via `Reverse`))

(fn `UserConstructionScript`)