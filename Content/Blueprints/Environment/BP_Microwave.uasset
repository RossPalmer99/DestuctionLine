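; BP_Microwave is an interactable microwave that swings its door open and spawns random food, and closes when damaged.
; A timeline rotates the hinge and toggles the door's Visibility collision.
; SpawnFood spawns an item from a random row of the FoodSpawnChance data table.
; A rare roll spawns food on every timeline update; otherwise DoOnce gates limit it to one item, with a single sound either way.
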(event `/Game/Data/Interact_Interface.Interact`
  (params (Player :type "/Game/Blueprints/Characters/Golem/0_Base Object Reference"))
  (set `self.SpawnsLoads` (> (`KismetMathLibrary.RandomIntegerInRange` 0 10) 9))
  (set `self.Open` true)
  (bind (_direction _rotation) (`Timeline|DoorAnimation` :!label _label)
    (:`Update`
      (`SceneComponent.K2_SetRelativeRotation` (`self.Hinge`) (`KismetMathLibrary.MakeRotator` 0.0 0.0 (* _rotation 140.0)) false false)
      (if (`self.Open`)
        (`PrimitiveComponent.SetCollisionResponseToChannel` (`self.Door`) "ECC_Visibility" "ECR_Ignore")
        (if (not (`self.SpawnsLoads`))
          (`/Engine/EditorBlueprintResources/StandardMacros.DoOnce` false :!label _label_2
            (:`Completed`
              _)))
        (`self.SpawnFood`)
        (`/Engine/EditorBlueprintResources/StandardMacros.DoOnce` false :!label _label_3
          (:`Completed`
            (`GameplayStatics.PlaySound2D` null 1.0 1.0 0.0 null null)))
        (else
          (`PrimitiveComponent.SetCollisionResponseToChannel` (`self.Door`) "ECC_Visibility" "ECR_Block")
          (`|ExecutionSequence`
            (:`then_0`
              (goto _label_2 :!via `Reset`))
            (:`then_1`
              (goto _label_3 :!via `Reset`))))))))

(event `self.ReceiveAnyDamage`
  (params (Damage :type "Float (single-precision)") (DamageType :type "DamageType Object Reference") (InstigatedBy :type "Controller Object Reference") (DamageCauser :type "Actor Object Reference"))
  (set `self.Open` false)
  (goto _label :!via `Reverse`))

(fn `SpawnFood`
  (returns (Food :type "Actor Object Reference"))
  (bind _returnvalue (`|GetDataTableRow` "/Game/Blueprints/Items/Data/FoodSpawnChance.FoodSpawnChance" (`KismetStringLibrary.Conv_StringToName` (`KismetStringLibrary.Conv_IntToString` (`KismetMathLibrary.RandomIntegerInRange` 0 32))))
    (:`then`
      (bind _returnvalue_2 (`|SpawnActorFromClass` (`.MicrowaveItems_25_7DEF36094858E9FD296E7C88695CBD73` (break `/Game/Blueprints/Items/Data/Struct_FoodArray` _returnvalue)) (`KismetMathLibrary.MakeTransform` (`self.K2_GetActorLocation`) (`self.K2_GetActorRotation`)) "Undefined" "OverrideRootScale" null null))
      (return _returnvalue_2))))

(fn `UserConstructionScript`)