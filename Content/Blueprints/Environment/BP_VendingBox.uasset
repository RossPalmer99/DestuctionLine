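; BP_VendingBox is an environment Blueprint for a vending box with a randomized colour scheme.
; On BeginPlay it sets its static mesh from the Boxes array, where the random range currently allows only the first entry.
; A single random index then picks matching PrimaryColours and SecondaryColours materials for the first two material slots, keeping each colour pair together.
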(event `self.ReceiveBeginPlay`
  (bind _staticmesh (`self.StaticMesh`))
  (`StaticMeshComponent.SetStaticMesh` (`self.StaticMesh`) (`|GetArrayItem` (`self.Boxes`) (`KismetMathLibrary.RandomIntegerInRange` 0)))
  (set `self.RandomInt` (`KismetMathLibrary.RandomIntegerInRange` 0 3))
  (`PrimitiveComponent.SetMaterial` _staticmesh 0 (`|GetArrayItem` (`self.PrimaryColours`) (`self.RandomInt`)))
  (`PrimitiveComponent.SetMaterial` _staticmesh 1 (`|GetArrayItem` (`self.SecondaryColours`) (`self.RandomInt`))))

(fn `UserConstructionScript`)