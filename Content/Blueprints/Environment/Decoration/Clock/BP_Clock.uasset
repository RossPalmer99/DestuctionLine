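; BP_Clock is a decorative analog clock that displays the real system time.
; Every tick it reads Now() and sets the relative pitch of the hour, minute and second hands, with milliseconds giving the second hand a smooth sweep.
; During evening and night hours it also swaps the face and hand materials on each tick, with no branch to restore daytime materials.
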(event `self.ReceiveTick`
  (params (DeltaSeconds :type "Float (single-precision)"))
  (bind _returnvalue (`KismetMathLibrary.Now`))
  (bind _clockface (`self.ClockFace`))
  (bind _returnvalue_2 (`KismetMathLibrary.GetHour` (`KismetMathLibrary.Now`)))
  (bind _returnvalue_3 (`KismetMathLibrary.GetMinute` _returnvalue))
  (bind _returnvalue_4 (`KismetMathLibrary.Conv_IntToDouble` (`KismetMathLibrary.GetSecond` _returnvalue)))
  (`SceneComponent.K2_SetRelativeRotation` (`self.HourHand`) (`KismetMathLibrary.MakeRotator` 0.0 (- 0.0 (* (+ (* (+ (* (`KismetMathLibrary.GetHour12` _returnvalue) 60.0) (`KismetMathLibrary.Conv_IntToDouble` _returnvalue_3)) 60.0) _returnvalue_4) 0.008333))) true false)
  (`SceneComponent.K2_SetRelativeRotation` (`self.MinuteHand`) (`KismetMathLibrary.MakeRotator` 0.0 (- 0.0 (* (+ (* _returnvalue_3 60.0) _returnvalue_4) 0.1))) true false)
  (`SceneComponent.K2_SetRelativeRotation` (`self.HourSecond`) (`KismetMathLibrary.MakeRotator` 0.0 (- 0.0 (* (+ (* (`KismetMathLibrary.GetMillisecond` _returnvalue) 0.001) _returnvalue_4) 6.0))) true false)
  (if (or (>= _returnvalue_2 20) (< _returnvalue_2 8))
    (`PrimitiveComponent.SetMaterial` _clockface 0 "/Game/Materials/Colours/M_cream.M_cream")
    (`PrimitiveComponent.SetMaterial` (`self.HourHand`) 0 "/Game/Materials/Colours/M_cream.M_cream")
    (`PrimitiveComponent.SetMaterial` (`self.MinuteHand`) 0 "/Game/Materials/Colours/M_cream.M_cream")
    (`PrimitiveComponent.SetMaterial` _clockface 1 "/Game/NEWASSETS/mat_black.mat_black")
    (`PrimitiveComponent.SetMaterial` (`self.HourSecond`) 0 "/Game/Materials/Colours/M_blue.M_blue")))

(fn `UserConstructionScript`)