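; Rotating red alarm light that switches on while a forklift spawner is triggered.
; Each Tick it finds all BP_ForkliftSpawner actors and, per spawner, sets the glow or dark material and both spotlights' visibility from IsTriggered.
; Each triggered spawner also yaws the Light component at a frame-rate-independent speed.
; With several spawners, the last one decides the on/off look and rotation steps add up.
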(event `self.ReceiveTick`
  (params (DeltaSeconds :type "Float (single-precision)"))
  (set `self.Delta` DeltaSeconds)
  (bind _outactors (`GameplayStatics.GetAllActorsOfClass` "/Game/Blueprints/RandomEvents/BP_ForkliftSpawner.BP_ForkliftSpawner_C"))
  (for _array_element _outactors
    (if (`/Game/Blueprints/RandomEvents/BP_ForkliftSpawner.IsTriggered` _array_element)
      (`PrimitiveComponent.SetMaterial` (`self.AlarmLightMesh`) 1 "/Game/Materials/Colours/M_red_glow.M_red_glow")
      (`SceneComponent.SetVisibility` (`self.SpotLight`) true false)
      (`SceneComponent.SetVisibility` (`self.SpotLight1`) true false)
      (bind _output_get (set `self.SpeedTest` (`self.Delta`)))
      (`SceneComponent.K2_AddRelativeRotation` (`self.Light`) (`KismetMathLibrary.MakeRotator` 0.0 0.0 (* _output_get 180.0)) false false)
      (else
        (`PrimitiveComponent.SetMaterial` (`self.AlarmLightMesh`) 1 "/Game/Materials/Colours/M_red_dark.M_red_dark")
        (`SceneComponent.SetVisibility` (`self.SpotLight`) false false)
        (`SceneComponent.SetVisibility` (`self.SpotLight1`) false false)))))

(fn `UserConstructionScript`)