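; BP_FLTEntrance is a forklift entrance that plays a one-shot open-close animation when the forklift spawner triggers.
; Each instance caches the spawner and all entrances on BeginPlay, then polls the spawner on Tick.
; DoOnce gates, reset when the trigger clears, activate the first two entrances in staggered order based on spawn side.
; A random forklift cue follows, occasionally with a tyre squeal.
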(event `self.ReceiveBeginPlay`
  (bind _outactors (`GameplayStatics.GetAllActorsOfClass` "/Game/Blueprints/RandomEvents/BP_ForkliftSpawner.BP_ForkliftSpawner_C"))
  (for _array_element _outactors
    _)
  (set `self.ForkliftSpawnerRef` _array_element)
  (bind _outactors_2 (`GameplayStatics.GetAllActorsOfClass` "BP_FLTEntrance_C"))
  (set `self.Entrances` _outactors_2))

(event `self.ReceiveTick`
  (params (DeltaSeconds :type "Float (single-precision)"))
  (if (`/Game/Blueprints/RandomEvents/BP_ForkliftSpawner.IsTriggered` (`self.ForkliftSpawnerRef`))
    (if (`/Game/Blueprints/RandomEvents/BP_ForkliftSpawner.RightSpawn` (`self.ForkliftSpawnerRef`))
      (`/Engine/EditorBlueprintResources/StandardMacros.DoOnce` false :!label _label
        (:`Completed`
          (`KismetSystemLibrary.Delay` 1.0)
          (`self.Activate` (`|GetArrayItem` (`self.Entrances`)))
          (`KismetSystemLibrary.Delay` 0.5)
          (`self.Activate` (`|GetArrayItem` (`self.Entrances`) 1))
          (`KismetSystemLibrary.Delay` 0.75)
          (if (`KismetMathLibrary.RandomBool`)
            (`GameplayStatics.PlaySound2D` "/Game/Audio/SFX/SE_Forklift_Cue.SE_Forklift_Cue" 1.0 1.0 0.0 null null)
            (if (== (`KismetMathLibrary.RandomIntegerInRange` 0 5) 5)
              (`GameplayStatics.PlaySound2D` "/Game/Audio/SFX/SE_TyreSqueal.SE_TyreSqueal" 1.0 1.0 0.0 null null)))))
      (else
        (`/Engine/EditorBlueprintResources/StandardMacros.DoOnce` false :!label _label_2
          (:`Completed`
            (`KismetSystemLibrary.Delay` 1.0)
            (`self.Activate` (`|GetArrayItem` (`self.Entrances`) 1))
            (`KismetSystemLibrary.Delay` 0.5)
            (`self.Activate` (`|GetArrayItem` (`self.Entrances`)))
            (`KismetSystemLibrary.Delay` 0.75)
            (if (`KismetMathLibrary.RandomBool`)
              (`GameplayStatics.PlaySound2D` "/Game/Audio/SFX/SE_Forklift_Cue.SE_Forklift_Cue" 1.0 1.0 0.0 null null)
              (if (== (`KismetMathLibrary.RandomIntegerInRange` 0 5) 5)
                (`GameplayStatics.PlaySound2D` "/Game/Audio/SFX/SE_TyreSqueal.SE_TyreSqueal" 1.0 1.0 0.0 null null)))))))
    (else
      (`|ExecutionSequence`
        (:`then_0`
          (goto _label :!via `Reset`))
        (:`then_1`
          (goto _label_2 :!via `Reset`))))))

(event `Activate`
  (`SkeletalMeshComponent.PlayAnimation` (`self.SkeletalMesh`) "/Game/Blueprints/Environment/Forklift_Entrance/OpenClose.OpenClose" false))

(fn `UserConstructionScript`)