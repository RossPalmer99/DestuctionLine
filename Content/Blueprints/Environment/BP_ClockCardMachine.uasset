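; BP_ClockCardMachine is an interactable clock card machine that launches the factory level.
; On Interact it sends the player a clocked-in message, then counts 0_Base actors flagged IsReady.
; When that count is exactly one, it saves through BP_GameInstance and opens the four-player factory map or the two-player variant, based on the game mode's MaxPlayerCount.
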(event `/Game/Data/Interact_Interface.Interact`
  (params (Player :type "/Game/Blueprints/Characters/Golem/0_Base Object Reference"))
  (message `/Game/Data/Interact_Interface.ClockedIn` Player self)
  (set `self.PlayersReady` 0)
  (bind _outactors (`GameplayStatics.GetAllActorsOfClass` "/Game/Blueprints/Characters/Golem/0_Base.0_Base_C"))
  (for _array_element _outactors
    (if (`/Game/Blueprints/Characters/Golem/0_Base.IsReady` _array_element)
      (set `self.PlayersReady` (+ (`self.PlayersReady`) 1))))
  (if (== (`self.PlayersReady`) 1)
    (bind _asbp_game_instance (cast `/Game/Data/BP_GameInstance` (`GameplayStatics.GetGameInstance`)))
    (`/Game/Data/BP_GameInstance.Save` _asbp_game_instance)
    (bind _asbp_gamemode (cast `/Game/Blueprints/Characters/BP_Gamemode` (`GameplayStatics.GetGameMode`)))
    (if (== (`/Game/Blueprints/Characters/BP_Gamemode.MaxPlayerCount` _asbp_gamemode) 4)
      (`GameplayStatics.OpenLevel` "map_Factory")
      (else
        (`GameplayStatics.OpenLevel` "map_2P_factory")))))

(fn `UserConstructionScript`)