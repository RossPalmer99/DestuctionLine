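; Vending machine environment actor that dispenses random actors on interaction and can be fractured by damage.
; Interact spawns one of the first two Actors entries at the Scene component's transform and records it in SpawnedActors.
; Once the added index exceeds 20, it removes the first entry, then destroys the actor that shifts into index 0.
; Any damage applies fixed radius damage to the Destructible component from the actor's location.
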(event `self.ReceiveAnyDamage`
  (params (Damage :type "Float (single-precision)") (DamageType :type "DamageType Object Reference") (InstigatedBy :type "Controller Object Reference") (DamageCauser :type "Actor Object Reference"))
  (`DestructibleComponent.ApplyRadiusDamage` (`self.Destructible`) 100.0 (`self.K2_GetActorLocation`) 0.0 0.0 false))

(event `/Game/Data/Interact_Interface.Interact`
  (params (Player :type "/Game/Blueprints/Characters/Golem/0_Base Object Reference"))
  (bind _spawnedactors (`self.SpawnedActors`))
  (bind _returnvalue (`|SpawnActorFromClass` (`|GetArrayItem` (`self.Actors`) (`KismetMathLibrary.RandomIntegerInRange` 0 1)) (`SceneComponent.K2_GetComponentToWorld` (`self.Scene`)) "Undefined" "OverrideRootScale" null null))
  (bind _returnvalue_2 (`KismetArrayLibrary.Array_Add` (`self.SpawnedActors`) _returnvalue))
  (if (> _returnvalue_2 20)
    (`KismetArrayLibrary.Array_Remove` _spawnedactors)
    (`self.K2_DestroyActor` (`|GetArrayItem` _spawnedactors))))

(fn `UserConstructionScript`)