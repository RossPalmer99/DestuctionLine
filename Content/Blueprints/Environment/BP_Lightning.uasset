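; Lightning actor that periodically appears, roams between TargetPoint actors and fires its Lightning effect.
; BeginPlay hides it, gathers all TargetPoints, appends "Lightning"-tagged ones again to the same array rather than filtering, and starts a looping timer.
; Each cycle, the Move timeline drives it forward while RInterpTo steers toward a random target, re-picked when close.
; When the timeline ends, it activates Lightning, then hides after short delays.
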(event `self.ReceiveBeginPlay`
  (bind _targetpoints (`self.TargetPoints`))
  (`self.SetActorHiddenInGame` true)
  (bind _outactors (`GameplayStatics.GetAllActorsOfClass` "/Script/Engine.TargetPoint"))
  (bind _output_get (set `self.TargetPoints` _outactors))
  (for _array_element _output_get
    (if (`self.ActorHasTag` _array_element "Lightning")
      (`KismetArrayLibrary.Array_Add` (`self.TargetPoints`) _array_element)))
  (set `self.CurrentTarget` (`|GetArrayItem` _targetpoints (`KismetMathLibrary.RandomIntegerInRange` 0 (`KismetArrayLibrary.Array_LastIndex` _targetpoints))))
  (`KismetSystemLibrary.K2_SetTimerDelegate` (delegate `MoveLightning`) 10.0 true))

(event `MoveLightning`
  (bind _targetpoints (`self.TargetPoints`))
  (`self.SetActorHiddenInGame` false)
  (`Timeline|Move` :!via `PlayFromStart`
    (:`Update`
      (`self.K2_SetActorLocationAndRotation` (+ (`self.K2_GetActorLocation`) (* (`self.GetActorForwardVector`) (`self.Speed`))) (`KismetMathLibrary.RInterpTo` (`self.K2_GetActorRotation`) (`KismetMathLibrary.FindLookAtRotation` (`self.K2_GetActorLocation`) (`self.K2_GetActorLocation` (`self.CurrentTarget`))) (`GameplayStatics.GetWorldDeltaSeconds`) 5.0))
      (if (< (`self.GetDistanceTo` (`self.CurrentTarget`)) 100.0)
        (set `self.CurrentTarget` (`|GetArrayItem` _targetpoints (`KismetMathLibrary.RandomIntegerInRange` 0 (`KismetArrayLibrary.Array_LastIndex` _targetpoints))))))
    (:`Finished`
      (`KismetSystemLibrary.Delay` 1.0)
      (`ActorComponent.Activate` (`self.Lightning`) false)
      (`KismetSystemLibrary.Delay` 1.0)
      (`self.SetActorHiddenInGame` true))))

(fn `UserConstructionScript`)