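; BP_ItemBin is a colour-coded bin that receives products players carry or throw into it.
; On BeginPlay it sets the bin material from BinInfo.Colour.
; Its collision overlap sets the player's ClosestBin and reports held or thrown products through ProductPlacedInBin or ProductThrownInBin, destroying them only when colours match.
; Ending the overlap clears the player's ClosestBin.
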(event `self.ReceiveBeginPlay`
  (bind _bininfo_colour (break `/Game/Blueprints/Environment/Struct_Bins` (`self.BinInfo`)))
  ;[1 1 1] SetColour
  (`self.CheckBinColour` _bininfo_colour))

(event `self.Collision.OnComponentBeginOverlap`
  (params (OverlappedComponent :type "PrimitiveComponent Object Reference") (OtherActor :type "Actor Object Reference") (OtherComp :type "PrimitiveComponent Object Reference") (OtherBodyIndex :type Integer) (bFromSweep :type Boolean) (SweepResult :type "HitResult Structure (by ref)"))
  (bind _bininfo_colour (break `/Game/Blueprints/Environment/Struct_Bins` (`self.BinInfo`)))
  (bind _bininfo_colour_2 (break `/Game/Blueprints/Environment/Struct_Bins` (`self.BinInfo`)))
  ;[1 1 1] Tell Player which bin this is
  (`|ExecutionSequence`
    (:`then_0`
      (bind _as0_base (cast `/Game/Blueprints/Characters/Golem/0_Base` OtherActor))
      (set `/Game/Blueprints/Characters/Golem/0_Base.ClosestBin` self _as0_base)
      (`/Engine/EditorBlueprintResources/StandardMacros.IsValid` _as0_base
        (:`Is Valid`
          (bind _helditem (`/Game/Blueprints/Characters/Golem/0_Base.HeldItem` _as0_base)
            (:`then`
              (bind _iteminfo_isproduct (break `/Game/Blueprints/Items/Data/Struct_ItemInfo` (`/Game/Blueprints/Items/BP_MasterItem.ItemInfo` _helditem)))
              (if _iteminfo_isproduct
                (bind _output_get (set `self.Product` _helditem))
                (`/Game/Blueprints/Characters/Golem/0_Base.ProductPlacedInBin` _as0_base)
                (bind (_iteminfo_isproduct_2 _iteminfo_isweapon1h _iteminfo_isweapon2h _iteminfo_isstacktruck _iteminfo_isfireextinguisher _iteminfo_isaccessory _iteminfo_ispowerup _iteminfo_isalarmclock _iteminfo_isbarrel _iteminfo_damage _iteminfo_weaponpower _iteminfo_weaponchip _iteminfo_colour) (break `/Game/Blueprints/Items/Data/Struct_ItemInfo` (`/Game/Blueprints/Items/BP_MasterItem.ItemInfo` _output_get)))
                (if (== _iteminfo_colour _bininfo_colour)
                  (`self.K2_DestroyActor` (`self.Product`))
                  (set `self.Product` null))))
            (:`else`)))))
    (:`then_1`
      (bind _asbp_product (cast `/Game/Blueprints/Items/BP_Product` OtherActor))
      (if (`/Game/Blueprints/Items/BP_MasterItem.HasBeenThrown` _asbp_product)
        (bind _throwingplayer (`/Game/Blueprints/Items/BP_Product.ThrowingPlayer` _asbp_product)
          (:`then`
            (set `/Game/Blueprints/Characters/Golem/0_Base.ClosestBin` self _throwingplayer)
            (`/Engine/EditorBlueprintResources/StandardMacros.IsValid` _throwingplayer
              (:`Is Valid`
                (`/Game/Blueprints/Characters/Golem/0_Base.ProductThrownInBin` _throwingplayer _asbp_product)
                (bind (_iteminfo_isproduct_3 _iteminfo_isweapon1h_2 _iteminfo_isweapon2h_2 _iteminfo_isstacktruck_2 _iteminfo_isfireextinguisher_2 _iteminfo_isaccessory_2 _iteminfo_ispowerup_2 _iteminfo_isalarmclock_2 _iteminfo_isbarrel_2 _iteminfo_damage_2 _iteminfo_weaponpower_2 _iteminfo_weaponchip_2 _iteminfo_colour_2) (break `/Game/Blueprints/Items/Data/Struct_ItemInfo` (`/Game/Blueprints/Items/BP_MasterItem.ItemInfo` _asbp_product)))
                (if (== _iteminfo_colour_2 _bininfo_colour_2)
                  (`self.K2_DestroyActor` _asbp_product)))))
          (:`else`))))))

(event `self.Collision.OnComponentEndOverlap`
  (params (OverlappedComponent :type "PrimitiveComponent Object Reference") (OtherActor :type "Actor Object Reference") (OtherComp :type "PrimitiveComponent Object Reference") (OtherBodyIndex :type Integer))
  ;[1 1 1] Tell Player which bin this is
  (bind _as0_base (cast `/Game/Blueprints/Characters/Golem/0_Base` OtherActor))
  (set `/Game/Blueprints/Characters/Golem/0_Base.ClosestBin` null _as0_base))

(fn `CheckBinColour`
  (params (Colour :type Name))
  (if (== Colour "Red")
    (`PrimitiveComponent.SetMaterial` (`self.Bin`) 0 "/Game/Materials/Colours/M_red_dark.M_red_dark")
    (return)
    (elif (== Colour "Green")
      (`PrimitiveComponent.SetMaterial` (`self.Bin`) 0 "/Game/Materials/Colours/M_green.M_green")
      (return)
      (elif (== Colour "Blue")
        (`PrimitiveComponent.SetMaterial` (`self.Bin`) 0 "/Game/Materials/Colours/M_blue_dark.M_blue_dark")
        (return)
        (elif (== Colour "Yellow")
          (`PrimitiveComponent.SetMaterial` (`self.Bin`) 0 "/Game/Materials/Colours/M_yellow.M_yellow")
          (return)
          (elif (== Colour "Grey")
            (`PrimitiveComponent.SetMaterial` (`self.Bin`) 0 "/Game/Materials/Colours/M_grey02.M_grey02")
            (return)))))))

(fn `UserConstructionScript`)