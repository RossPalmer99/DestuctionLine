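; BP_CrateSpawner is a placed actor that periodically spawns deathmatch crates at its own location and rotation.
; On BeginPlay it starts a looping SpawnEither timer, with an interval randomized once between 20 and 30 seconds.
; SpawnEither flips the IsWeapon flag to alternate between BP_DM_WeaponCrate and BP_DM_PowerCrate.
; Separate SpawnWeapon and SpawnPowerUP functions exist, but their timer setups are disconnected.
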(event `self.ReceiveBeginPlay`
  (`KismetSystemLibrary.K2_SetTimer` null "SpawnEither" (`KismetMathLibrary.RandomFloatInRange` 20.0 30.0) true))

(fn `SpawnEither`
  (if (`self.IsWeapon`)
    (`|SpawnActorFromClass` "/Game/Blueprints/DestructibleBlueprints/BP_DM_WeaponCrate.BP_DM_WeaponCrate_C" (`KismetMathLibrary.MakeTransform` (`self.K2_GetActorLocation`) (`self.K2_GetActorRotation`)) "Undefined" "OverrideRootScale" null null)
    (set `self.IsWeapon` false)
    (else
      (`|SpawnActorFromClass` "/Game/Blueprints/DestructibleBlueprints/BP_DM_PowerCrate.BP_DM_PowerCrate_C" (`KismetMathLibrary.MakeTransform` (`self.K2_GetActorLocation`) (`self.K2_GetActorRotation`)) "Undefined" "OverrideRootScale" null null)
      (set `self.IsWeapon` true))))

(fn `SpawnPowerUP`
  (`|SpawnActorFromClass` "/Game/Blueprints/DestructibleBlueprints/BP_DM_PowerCrate.BP_DM_PowerCrate_C" (`KismetMathLibrary.MakeTransform` (`self.K2_GetActorLocation`) (`self.K2_GetActorRotation`)) "Undefined" "OverrideRootScale" null null))

(fn `SpawnWeapon`
  (`|SpawnActorFromClass` "/Game/Blueprints/DestructibleBlueprints/BP_DM_WeaponCrate.BP_DM_WeaponCrate_C" (`KismetMathLibrary.MakeTransform` (`self.K2_GetActorLocation`) (`self.K2_GetActorRotation`)) "Undefined" "OverrideRootScale" null null))

(fn `UserConstructionScript`)