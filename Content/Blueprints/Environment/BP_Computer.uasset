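; Interactable computer prop that shows an assigned camera texture on its monitor and lets a player sit on it with a calling card HUD.
; AssignCamera feeds the texture into a dynamic material instance on the monitor.
; Interact uses a FlipFlop to enter or leave, toggling the player's movement and IsOnComputer flag while tracking the user.
; Each player's WBP_CallingCard is anchored to a screen corner chosen by matching hardcoded player display names.
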(event `/Game/Data/Interact_Interface.AssignCamera`
  (params (ScreenTexture :type "TextureRenderTarget2D Object Reference") (CCTV :type "/Game/Blueprints/CameraSystem/CCTV/BP_CCTV Object Reference"))
  (set `self.Texture` ScreenTexture)
  (bind _returnvalue (`PrimitiveComponent.CreateDynamicMaterialInstance` (`self.Monitor`) 0 "/Game/Blueprints/CameraSystem/CCTV/M_Monitor_Normal.M_Monitor_Normal" "None"))
  (bind _output_get (set `self.MIDTVScreen` _returnvalue))
  (`MaterialInstanceDynamic.SetTextureParameterValue` _output_get "ScreenTexture01" (`self.Texture`)))

(event `/Game/Data/Interact_Interface.Interact`
  (params (Player :type "/Game/Blueprints/Characters/Golem/0_Base Object Reference"))
  (bind _arrayofhuds (`self.ArrayOfHUDs`))
  (bind _output_get (set `self.NewInteracter` Player))
  (if (== _output_get (`self.PlayerUsingComputer`))
    (`/Engine/EditorBlueprintResources/StandardMacros.FlipFlop` :!label _label
      (:`A`
        (`KismetArrayLibrary.Array_Add` (`self.ArrayOfPlayers`) Player)
        (bind _returnvalue (`|CreateWidget` "/Game/Blueprints/Characters/WBPs/WBP_CallingCard.WBP_CallingCard_C" null (`/Game/Blueprints/Characters/Golem/0_Base.Index` Player)))
        (`KismetArrayLibrary.Array_Add` (`self.ArrayOfHUDs`) _returnvalue)
        (`UserWidget.AddToViewport` _returnvalue 0)
        (bind _returnvalue_2 (`WidgetLayoutLibrary.SlotAsCanvasSlot` (`/Game/Blueprints/Characters/WBPs/WBP_CallingCard.Border_0` _returnvalue)))
        (`KismetArrayLibrary.Array_Add` (`self.ArrayOfHUDSlots`) _returnvalue_2)
        (switch `string` (`KismetSystemLibrary.GetDisplayName` Player)
          (:`0_Base`
            (set `self.HUDMinAnchors` (0.0 0.0))
            (set `self.HUDMaxAnchors` (0.0 0.0))
            (set `self.HUDXPos` 50.0)
            (set `self.HUDYPos` 50.0))
          (:`0_Base1`
            (set `self.HUDMinAnchors` (1.0 0.0))
            (set `self.HUDMaxAnchors` (1.0 0.0))
            (set `self.HUDXPos` -620.0)
            (set `self.HUDYPos` 50.0))
          (:`0_Base2`
            (set `self.HUDMinAnchors` (0.0 1.0))
            (set `self.HUDMaxAnchors` (0.0 1.0))
            (set `self.HUDXPos` 50.0)
            (set `self.HUDYPos` -620.0))
          (:`0_Base3`
            (set `self.HUDMinAnchors` (1.0 1.0))
            (set `self.HUDMaxAnchors` (1.0 1.0))
            (set `self.HUDXPos` -620.0)
            (set `self.HUDYPos` -620.0)))
        (`CanvasPanelSlot.SetAnchors` _returnvalue_2 (make `Anchors` (`self.HUDMinAnchors`) (`self.HUDMaxAnchors`)))
        (`CanvasPanelSlot.SetPosition` _returnvalue_2 (`KismetMathLibrary.MakeVector2D` (`self.HUDXPos`) (`self.HUDYPos`)))
        (bind _output_get_2 (set `self.PlayerUsingComputer` Player))
        (`CharacterMovementComponent.DisableMovement` (`Character.CharacterMovement` _output_get_2))
        (set `/Game/Blueprints/Characters/Golem/0_Base.IsOnComputer` true Player))
      (:`B`
        (for (_array_element _array_index) (`self.ArrayOfPlayers`)
          (if (`KismetStringLibrary.EqualEqual_StrStr` (`KismetSystemLibrary.GetDisplayName` _array_element) (`KismetSystemLibrary.GetDisplayName` Player))
            (`KismetArrayLibrary.Array_Remove` (`self.ArrayOfPlayers`) _array_index)
            (`Widget.RemoveFromParent` (`|GetArrayItem` _arrayofhuds _array_index))
            (`KismetArrayLibrary.Array_Remove` _arrayofhuds _array_index)
            (`KismetArrayLibrary.Array_Remove` (`self.ArrayOfHUDSlots`) _array_index)
            (`CharacterMovementComponent.SetMovementMode` (`Character.CharacterMovement` (`self.PlayerUsingComputer`)) "MOVE_Walking" 0)
            (set `self.PlayerUsingComputer` null)
            (set `/Game/Blueprints/Characters/Golem/0_Base.IsOnComputer` false Player)))))
    (elif (== (`self.PlayerUsingComputer`) null)
      (goto _label))))

(fn `UserConstructionScript`)