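; BP_ExitDoor is an exit door that offers the exit menu to a player who interacts with it from inside its trigger Box.
; Interact stores the player, confirms the overlap, then sends ExitMenuMessage with the player's index and the door to that player's controller.
; Box begin and end overlaps from 0_Base actors swap an ExitSign material between an emissive green and the standard exit-sign green.
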(event `/Game/Data/Interact_Interface.Interact`
  (params (Player :type "/Game/Blueprints/Characters/Golem/0_Base Object Reference"))
  (set `self.PlayerRef` Player)
  (if (`PrimitiveComponent.IsOverlappingActor` (`self.Box`) Player)
    (message `/Game/Data/Interact_Interface.ExitMenu` (`GameplayStatics.GetPlayerController` (`/Game/Blueprints/Characters/Golem/0_Base.Index` Player)) (`/Game/Blueprints/Characters/Golem/0_Base.Index` Player) self)))

(event `self.Box.OnComponentBeginOverlap`
  (params (OverlappedComponent :type "PrimitiveComponent Object Reference") (OtherActor :type "Actor Object Reference") (OtherComp :type "PrimitiveComponent Object Reference") (OtherBodyIndex :type Integer) (bFromSweep :type Boolean) (SweepResult :type "HitResult Structure (by ref)"))
  (cast `/Game/Blueprints/Characters/Golem/0_Base` OtherActor)
  (`PrimitiveComponent.SetMaterial` (`self.ExitSign`) 1 "/Game/Materials/Colours/M_green_emissive.M_green_emissive"))

(event `self.Box.OnComponentEndOverlap`
  (params (OverlappedComponent :type "PrimitiveComponent Object Reference") (OtherActor :type "Actor Object Reference") (OtherComp :type "PrimitiveComponent Object Reference") (OtherBodyIndex :type Integer))
  (cast `/Game/Blueprints/Characters/Golem/0_Base` OtherActor)
  (`PrimitiveComponent.SetMaterial` (`self.ExitSign`) 1 "/Game/Materials/Colours/M_green_exitsign.M_green_exitsign"))

(fn `UserConstructionScript`)