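; BP_Incinerator is an environment hazard that sets products and players on fire when they enter its box trigger.
; Each overlap stores the product or player, replacing any previous one, and starts a looping named-function timer.
; The timers repeatedly call OnFire: unconditionally on a valid product, but on the player only while still overlapping the box.
; Nothing in the file clears the timers or resets the burning flag.
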(event `self.ReceiveBeginPlay`)

(event `self.Box.OnComponentBeginOverlap`
  (params (OverlappedComponent :type "PrimitiveComponent Object Reference") (OtherActor :type "Actor Object Reference") (OtherComp :type "PrimitiveComponent Object Reference") (OtherBodyIndex :type Integer) (bFromSweep :type Boolean) (SweepResult :type "HitResult Structure (by ref)"))
  (`|ExecutionSequence`
    (:`then_0`
      (bind _asbp_product (cast `/Game/Blueprints/Items/BP_Product` OtherActor))
      (set `self.Product` _asbp_product)
      (`KismetSystemLibrary.K2_SetTimer` null "BoxesOnFire" 0.1 true))
    (:`then_1`
      (bind _as0_base (cast `/Game/Blueprints/Characters/Golem/0_Base` OtherActor))
      (set `self.Player` _as0_base)
      (`KismetSystemLibrary.K2_SetTimer` null "PlayersOnFire" 0.1 true))))

(fn `BoxesOnFire`
  (bind _product (`self.Product`)
    (:`then`
      (`/Game/Blueprints/Items/BP_Product.OnFire` _product))
    (:`else`)))

(fn `PlayersOnFire`
  (bind _player (`self.Player`)
    (:`then`
      (if (`PrimitiveComponent.IsOverlappingActor` (`self.Box`) _player)
        (bind _output_get (set `self.PlayerOnFire` true))
        (`/Game/Blueprints/Characters/Golem/0_Base.OnFire` (`self.Player`) _output_get)))
    (:`else`)))

(fn `UserConstructionScript`)