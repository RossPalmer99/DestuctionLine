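; Product spawner for a player corner that periodically spawns coloured BP_Product actors.
; BeginPlay spawns a non-simulating template product, then calls Spawn immediately and on a looping timer whose random interval is rolled once.
; Spawn picks a random ProductColourChance row within SpawnChance, maps its relative colour to a real one for the PlayerCorner, and copies the template's item and power info.
; Each product receives a reference back to its spawner.
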(event `self.ReceiveBeginPlay`
  (bind _returnvalue (`SceneComponent.K2_GetComponentToWorld` (`self.DefaultSceneRoot`)))
  (bind _returnvalue_2 (`|SpawnActorFromClass` "/Game/Blueprints/Items/BP_Product.BP_Product_C" (`KismetMathLibrary.MakeTransform` (`self.BoxRefSpawnLoc`) (.rotation _returnvalue) (.scale _returnvalue)) "Undefined" "OverrideRootScale" null (struct) (struct) false "NewEnumerator0" null))
  (`PrimitiveComponent.SetSimulatePhysics` (`/Game/Blueprints/Items/BP_MasterItem.StaticMesh` _returnvalue_2) false)
  (set `self.ProductDefault` _returnvalue_2)
  (`self.spawn`)
  (`KismetSystemLibrary.K2_SetTimer` null "Spawn" (`KismetMathLibrary.RandomFloatInRange` 10.0 12.0) true))

(fn `SetColours`
  (params (ColourIn :type Name))
  (returns (ColourOut :type Name))
  (if (== (`self.PlayerCorner`) 0)
    (bind _colourout (`self.SetColoursP0` (`KismetStringLibrary.Conv_NameToString` ColourIn)))
    (return _colourout)
    (elif (== (`self.PlayerCorner`) 1)
      (bind _colourout_2 (`self.SetColoursP1` (`KismetStringLibrary.Conv_NameToString` ColourIn)))
      (return _colourout_2)
      (elif (== (`self.PlayerCorner`) 2)
        (bind _colourout_3 (`self.SetColoursP2` (`KismetStringLibrary.Conv_NameToString` ColourIn)))
        (return _colourout_3)
        (elif (== (`self.PlayerCorner`) 3)
          (bind _colourout_4 (`self.SetColoursP3` (`KismetStringLibrary.Conv_NameToString` ColourIn)))
          (return _colourout_4))))))

(fn `SetColoursP0`
  (params (ColourIn :type String))
  (returns (ColourOut :type Name))
  (if (`KismetStringLibrary.EqualEqual_StrStr` ColourIn "MyColour")
    (return (`KismetStringLibrary.Conv_StringToName` (`KismetStringLibrary.Replace` ColourIn "MyColour" "Red" "CaseSensitive")))
    (elif (`KismetStringLibrary.EqualEqual_StrStr` ColourIn "AltColour1")
      (return (`KismetStringLibrary.Conv_StringToName` (`KismetStringLibrary.Replace` ColourIn "AltColour1" "Green" "CaseSensitive")))
      (elif (`KismetStringLibrary.EqualEqual_StrStr` ColourIn "AltColour2")
        (return (`KismetStringLibrary.Conv_StringToName` (`KismetStringLibrary.Replace` ColourIn "AltColour2" "Blue" "CaseSensitive")))
        (elif (`KismetStringLibrary.EqualEqual_StrStr` ColourIn "AltColour3")
          (return (`KismetStringLibrary.Conv_StringToName` (`KismetStringLibrary.Replace` ColourIn "AltColour3" "Yellow" "CaseSensitive")))
          (elif (`KismetStringLibrary.EqualEqual_StrStr` ColourIn "Grey")
            (return (`KismetStringLibrary.Conv_StringToName` ColourIn))))))))

(fn `SetColoursP1`
  (params (ColourIn :type String))
  (returns (ColourOut :type Name))
  (if (`KismetStringLibrary.EqualEqual_StrStr` ColourIn "MyColour")
    (return (`KismetStringLibrary.Conv_StringToName` (`KismetStringLibrary.Replace` ColourIn "MyColour" "Green" "CaseSensitive")))
    (elif (`KismetStringLibrary.EqualEqual_StrStr` ColourIn "AltColour1")
      (return (`KismetStringLibrary.Conv_StringToName` (`KismetStringLibrary.Replace` ColourIn "AltColour1" "Red" "CaseSensitive")))
      (elif (`KismetStringLibrary.EqualEqual_StrStr` ColourIn "AltColour2")
        (return (`KismetStringLibrary.Conv_StringToName` (`KismetStringLibrary.Replace` ColourIn "AltColour2" "Blue" "CaseSensitive")))
        (elif (`KismetStringLibrary.EqualEqual_StrStr` ColourIn "AltColour3")
          (return (`KismetStringLibrary.Conv_StringToName` (`KismetStringLibrary.Replace` ColourIn "AltColour3" "Yellow" "CaseSensitive")))
          (elif (`KismetStringLibrary.EqualEqual_StrStr` ColourIn "Grey")
            (return (`KismetStringLibrary.Conv_StringToName` ColourIn))))))))

(fn `SetColoursP2`
  (params (ColourIn :type String))
  (returns (ColourOut :type Name))
  (if (`KismetStringLibrary.EqualEqual_StrStr` ColourIn "MyColour")
    (return (`KismetStringLibrary.Conv_StringToName` (`KismetStringLibrary.Replace` ColourIn "MyColour" "Blue" "CaseSensitive")))
    (elif (`KismetStringLibrary.EqualEqual_StrStr` ColourIn "AltColour1")
      (return (`KismetStringLibrary.Conv_StringToName` (`KismetStringLibrary.Replace` ColourIn "AltColour1" "Red" "CaseSensitive")))
      (elif (`KismetStringLibrary.EqualEqual_StrStr` ColourIn "AltColour2")
        (return (`KismetStringLibrary.Conv_StringToName` (`KismetStringLibrary.Replace` ColourIn "AltColour2" "Green" "CaseSensitive")))
        (elif (`KismetStringLibrary.EqualEqual_StrStr` ColourIn "AltColour3")
          (return (`KismetStringLibrary.Conv_StringToName` (`KismetStringLibrary.Replace` ColourIn "AltColour3" "Yellow" "CaseSensitive")))
          (elif (`KismetStringLibrary.EqualEqual_StrStr` ColourIn "Grey")
            (return (`KismetStringLibrary.Conv_StringToName` ColourIn))))))))

(fn `SetColoursP3`
  (params (ColourIn :type String))
  (returns (ColourOut :type Name))
  (if (`KismetStringLibrary.EqualEqual_StrStr` ColourIn "MyColour")
    (return (`KismetStringLibrary.Conv_StringToName` (`KismetStringLibrary.Replace` ColourIn "MyColour" "Yellow" "CaseSensitive")))
    (elif (`KismetStringLibrary.EqualEqual_StrStr` ColourIn "AltColour1")
      (return (`KismetStringLibrary.Conv_StringToName` (`KismetStringLibrary.Replace` ColourIn "AltColour1" "Red" "CaseSensitive")))
      (elif (`KismetStringLibrary.EqualEqual_StrStr` ColourIn "AltColour2")
        (return (`KismetStringLibrary.Conv_StringToName` (`KismetStringLibrary.Replace` ColourIn "AltColour2" "Green" "CaseSensitive")))
        (elif (`KismetStringLibrary.EqualEqual_StrStr` ColourIn "AltColour3")
          (return (`KismetStringLibrary.Conv_StringToName` (`KismetStringLibrary.Replace` ColourIn "AltColour3" "Blue" "CaseSensitive")))
          (elif (`KismetStringLibrary.EqualEqual_StrStr` ColourIn "Grey")
            (return (`KismetStringLibrary.Conv_StringToName` ColourIn))))))))

(fn `spawn`
  (locals (MyColour :type String))
  (bind (_returnvalue_roll _returnvalue_pitch _returnvalue_yaw) (`KismetMathLibrary.BreakRotator` (`KismetMathLibrary.RandomRotator` false)))
  (bind _productdefault (`self.ProductDefault`))
  (bind (_iteminfo_isproduct _iteminfo_isweapon1h _iteminfo_isweapon2h _iteminfo_isstacktruck _iteminfo_isfireextinguisher _iteminfo_isaccessory _iteminfo_ispowerup _iteminfo_isalarmclock _iteminfo_isbarrel _iteminfo_damage _iteminfo_weaponpower _iteminfo_weaponchip _iteminfo_colour _iteminfo_pointvalue) (break `/Game/Blueprints/Items/Data/Struct_ItemInfo` (`/Game/Blueprints/Items/BP_MasterItem.ItemInfo` _productdefault)))
  (bind _returnvalue (`|GetDataTableRow` "/Game/Blueprints/Items/Data/ProductColourChance.ProductColourChance" (`KismetStringLibrary.Conv_StringToName` (`KismetStringLibrary.Conv_IntToString` (`KismetMathLibrary.RandomIntegerInRange` 0 (`self.SpawnChance`)))))
    (:`then`
      (bind _colourout (`self.SetColours` (`.Colour_5_7DEF36094858E9FD296E7C88695CBD73` (break `/Game/Blueprints/Items/Data/Struct_ColourArray` _returnvalue))))
      (set `self.Colour` _colourout)
      (bind _returnvalue_2 (`|SpawnActorFromClass` "/Game/Blueprints/Items/BP_Product.BP_Product_C" (`KismetMathLibrary.MakeTransform` (`self.K2_GetActorLocation`) (`KismetMathLibrary.MakeRotator` 0.0 0.0 _returnvalue_yaw) (1.0 1.0 1.0)) "Undefined" "OverrideRootScale" null (make `/Game/Blueprints/Items/Data/Struct_ItemInfo` _iteminfo_isproduct _iteminfo_isweapon1h _iteminfo_isweapon2h _iteminfo_isstacktruck _iteminfo_isfireextinguisher _iteminfo_isaccessory _iteminfo_ispowerup _iteminfo_isalarmclock _iteminfo_isbarrel _iteminfo_damage _iteminfo_weaponpower _iteminfo_weaponchip (`self.Colour`) _iteminfo_pointvalue) (`/Game/Blueprints/Items/BP_MasterItem.PowerInfo` _productdefault) false "NewEnumerator0" null))
      (set `/Game/Blueprints/Items/BP_Product.Spawner` self _returnvalue_2))))

(fn `UserConstructionScript`)