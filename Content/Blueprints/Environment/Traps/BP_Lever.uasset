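; BP_Lever is an interactable lever that toggles its referenced trap on or off.
; On Interact it checks TrapActivated, calls ActivateTrap or DeactivateTrap accordingly, then runs PullLever.
; PullLever drives LeverRotator's pitch with a timeline and reverses it on finish, with a DoOnce, reset each pull, limiting the return swing to once.
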(event `/Game/Data/Interact_Interface.Interact`
  (params (Player :type "/Game/Blueprints/Characters/Golem/0_Base Object Reference"))
  ;[1 1 1] Lever Interaction
  (set `self.Player` Player)
  (if (`/Game/Blueprints/Environment/Traps/BP_Trap.TrapActivated` (`self.Traps`))
    (`/Game/Blueprints/Environment/Traps/BP_Trap.DeactivateTrap` (`self.Traps`))
    (`self.PullLever`)
    (else
      (`/Game/Blueprints/Environment/Traps/BP_Trap.ActivateTrap` (`self.Traps`))
      (`self.PullLever`))))

(event `PullLever`
  ;[1 1 1] Lever Animation
  (`|ExecutionSequence`
    (:`then_0`
      (bind (_direction _y) (`Timeline|LeverRotation`)
        (:`Update`
          (`SceneComponent.K2_SetRelativeRotation` (`self.LeverRotator`) (`KismetMathLibrary.MakeRotator` 0.0 _y) false false))
        (:`Finished`
          (`/Engine/EditorBlueprintResources/StandardMacros.DoOnce` false :!label _label
            (:`Completed`
              (`TimelineComponent.Reverse` (`self.LeverRotation`)))))))
    (:`then_1`
      (goto _label :!via `Reset`))))

(fn `UserConstructionScript`)