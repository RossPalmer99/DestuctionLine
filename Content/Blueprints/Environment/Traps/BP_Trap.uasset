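; BP_Trap is an environment trap with two sliding doors and a spring that launches and damages actors.
; ActivateTrap plays the left and right door timelines to slide the doors open, and DeactivateTrap reverses them to close.
; Independently of the door state, overlapping SpringCollision waits briefly, fires a RadialForce impulse, then applies damage to every actor overlapping TestArea.
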(event `DeactivateTrap`
  ;[1 1 1] Close Doors
  (set `self.TrapActivated` false)
  (`|ExecutionSequence`
    (:`then_0`
      (`TimelineComponent.Reverse` (`self.LeftDoorAnimations`)))
    (:`then_1`
      (`TimelineComponent.Reverse` (`self.RightDoorAnimations`)))))

(event `ActivateTrap`
  ;[1 1 1] Open Doors
  (set `self.TrapActivated` true)
  (`|ExecutionSequence`
    (:`then_0`
      (bind (_direction _x_location) (`Timeline|LeftDoorAnimations`)
        (:`Update`
          (`SceneComponent.K2_SetRelativeLocation` (`self.TrapDoorLeft`) (`KismetMathLibrary.MakeVector` _x_location 0.1) false false))
        (:`Finished`
          (`/Engine/EditorBlueprintResources/StandardMacros.DoOnce` false :!label _label))))
    (:`then_1`
      (goto _label :!via `Reset`))
    (:`then_2`
      (bind (_direction_2 _x_location_2) (`Timeline|RightDoorAnimations`)
        (:`Update`
          (`SceneComponent.K2_SetRelativeLocation` (`self.TrapDoorRight`) (`KismetMathLibrary.MakeVector` _x_location_2 0.1) false false))
        (:`Finished`
          (`/Engine/EditorBlueprintResources/StandardMacros.DoOnce` false :!label _label_2))))
    (:`then_3`
      (goto _label_2 :!via `Reset`))))

(event `self.SpringCollision.OnComponentBeginOverlap`
  (params (OverlappedComponent :type "PrimitiveComponent Object Reference") (OtherActor :type "Actor Object Reference") (OtherComp :type "PrimitiveComponent Object Reference") (OtherBodyIndex :type Integer) (bFromSweep :type Boolean) (SweepResult :type "HitResult Structure (by ref)"))
  (`KismetSystemLibrary.Delay` 1.0)
  (`RadialForceComponent.FireImpulse` (`self.RadialForce`))
  (for _array_element (`PrimitiveComponent.GetOverlappingActors` (`self.TestArea`) null)
    (`GameplayStatics.ApplyDamage` _array_element 10.0 null self)))

(fn `UserConstructionScript`)