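; BP_Coffin is a graveyard coffin that bursts apart and releases an AI zombie.
; A timed BeginPlay sequence fractures the front destructible pieces with radius damage, then spawns BP_Zombie running BT_ZombieAI at the coffin's location.
; It then breaks the main body the same way and destroys the actor once a final delay has passed.
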(event `self.ReceiveBeginPlay`
  (`KismetSystemLibrary.Delay` 2.0)
  (`DestructibleComponent.ApplyRadiusDamage` (`self.GraveyardAssets_model_coffin_front_1_polySurface2_DM`) 100.0 (`self.K2_GetActorLocation`) 200.0 100.0 true)
  (`DestructibleComponent.ApplyRadiusDamage` (`self.GraveyardAssets_model_coffin_front_1_polySurface1_DM`) 100.0 (`self.K2_GetActorLocation`) 200.0 100.0 true)
  (`KismetSystemLibrary.Delay` 0.5)
  (`AIBlueprintHelperLibrary.SpawnAIFromClass` "/Game/Blueprints/AI/ZombieAI/BP_Zombie.BP_Zombie_C" "/Game/Blueprints/AI/ZombieAI/BT_ZombieAI.BT_ZombieAI" (`self.K2_GetActorLocation`) (struct) true)
  (`KismetSystemLibrary.Delay` 2.0)
  (`DestructibleComponent.ApplyRadiusDamage` (`self.GraveyardAssets_model_coffin_main_DM`) 100.0 (`self.K2_GetActorLocation`) 200.0 100.0 true)
  (`KismetSystemLibrary.Delay` 10.0)
  (`self.K2_DestroyActor`))

(fn `UserConstructionScript`)