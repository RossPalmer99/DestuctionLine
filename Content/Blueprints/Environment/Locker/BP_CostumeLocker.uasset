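; Costume locker that lets up to four local players browse and change their character outfit.
; Interact opens a WBP_Locker per player in its screen corner, previewing outfits through that player's HudCharacter and material.
; CycleMenu steps through ArrayOfOutfits per player, Confirm applies the mesh and saves it to PlayerInfo, and leaving InteractArea closes the widget.
; Players are told apart by actor display name, with duplicated logic for each slot.
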(event `/Game/Data/Interact_Interface.Confirm`
  (params (Player :type "/Game/Blueprints/Characters/Golem/0_Base Object Reference"))
  (bind (_playerinfo_playername _playerinfo_rank _playerinfo_items_crafted _playerinfo_products_shipped _playerinfo_tasks_completed _playerinfo_players_knocked_out _playerinfo_players_knocked_out_unarmed _playerinfo_players_knocked_out_1h _playerinfo_players_knocked_out_2h _playerinfo_players_knocked_out_sp _playerinfo_players_knocked_out_ra _playerinfo_times_taunted _playerinfo_pointsround) (break `/Game/Blueprints/Characters/Golem/Struct_PlayerInfo` (`/Game/Blueprints/Characters/Golem/0_Base.PlayerInfo` Player)))
  (bind (_playerinfo_playername_2 _playerinfo_rank_2 _playerinfo_items_crafted_2 _playerinfo_products_shipped_2 _playerinfo_tasks_completed_2 _playerinfo_players_knocked_out_2 _playerinfo_players_knocked_out_unarmed_2 _playerinfo_players_knocked_out_1h_2 _playerinfo_players_knocked_out_2h_2 _playerinfo_players_knocked_out_sp_2 _playerinfo_players_knocked_out_ra_2 _playerinfo_times_taunted_2 _playerinfo_pointsround_2) (break `/Game/Blueprints/Characters/Golem/Struct_PlayerInfo` (`/Game/Blueprints/Characters/Golem/0_Base.PlayerInfo` Player)))
  (bind (_playerinfo_playername_3 _playerinfo_rank_3 _playerinfo_items_crafted_3 _playerinfo_products_shipped_3 _playerinfo_tasks_completed_3 _playerinfo_players_knocked_out_3 _playerinfo_players_knocked_out_unarmed_3 _playerinfo_players_knocked_out_1h_3 _playerinfo_players_knocked_out_2h_3 _playerinfo_players_knocked_out_sp_3 _playerinfo_players_knocked_out_ra_3 _playerinfo_times_taunted_3 _playerinfo_pointsround_3) (break `/Game/Blueprints/Characters/Golem/Struct_PlayerInfo` (`/Game/Blueprints/Characters/Golem/0_Base.PlayerInfo` Player)))
  (bind (_playerinfo_playername_4 _playerinfo_rank_4 _playerinfo_items_crafted_4 _playerinfo_products_shipped_4 _playerinfo_tasks_completed_4 _playerinfo_players_knocked_out_4 _playerinfo_players_knocked_out_unarmed_4 _playerinfo_players_knocked_out_1h_4 _playerinfo_players_knocked_out_2h_4 _playerinfo_players_knocked_out_sp_4 _playerinfo_players_knocked_out_ra_4 _playerinfo_times_taunted_4 _playerinfo_pointsround_4) (break `/Game/Blueprints/Characters/Golem/Struct_PlayerInfo` (`/Game/Blueprints/Characters/Golem/0_Base.PlayerInfo` Player)))
  (bind _skeletalmesh (`SkinnedMeshComponent.SkeletalMesh` (`/Game/Blueprints/Environment/Locker/BP_HudCharacter.SkeletalMesh` (`self.HudCharacter3`))))
  (bind _skeletalmesh_2 (`SkinnedMeshComponent.SkeletalMesh` (`/Game/Blueprints/Environment/Locker/BP_HudCharacter.SkeletalMesh` (`self.HudCharacter0`))))
  (bind _skeletalmesh_3 (`SkinnedMeshComponent.SkeletalMesh` (`/Game/Blueprints/Environment/Locker/BP_HudCharacter.SkeletalMesh` (`self.HudCharacter1`))))
  (bind _skeletalmesh_4 (`SkinnedMeshComponent.SkeletalMesh` (`/Game/Blueprints/Environment/Locker/BP_HudCharacter.SkeletalMesh` (`self.HudCharacter2`))))
  (switch `string` (`KismetSystemLibrary.GetDisplayName` Player)
    (:`0_Base`
      (message `/Game/Data/Interact_Interface.ChangeOutfit` Player _skeletalmesh_2)
      (set `/Game/Blueprints/Characters/Golem/0_Base.PlayerInfo` (make `/Game/Blueprints/Characters/Golem/Struct_PlayerInfo` _playerinfo_playername_2 _playerinfo_rank_2 _playerinfo_items_crafted_2 _playerinfo_products_shipped_2 _playerinfo_tasks_completed_2 _playerinfo_players_knocked_out_2 _playerinfo_players_knocked_out_unarmed_2 _playerinfo_players_knocked_out_1h_2 _playerinfo_players_knocked_out_2h_2 _playerinfo_players_knocked_out_sp_2 _playerinfo_players_knocked_out_ra_2 _playerinfo_times_taunted_2 _playerinfo_pointsround_2 _skeletalmesh_2) Player))
    (:`0_Base1`
      (message `/Game/Data/Interact_Interface.ChangeOutfit` Player _skeletalmesh_3)
      (set `/Game/Blueprints/Characters/Golem/0_Base.PlayerInfo` (make `/Game/Blueprints/Characters/Golem/Struct_PlayerInfo` _playerinfo_playername_4 _playerinfo_rank_4 _playerinfo_items_crafted_4 _playerinfo_products_shipped_4 _playerinfo_tasks_completed_4 _playerinfo_players_knocked_out_4 _playerinfo_players_knocked_out_unarmed_4 _playerinfo_players_knocked_out_1h_4 _playerinfo_players_knocked_out_2h_4 _playerinfo_players_knocked_out_sp_4 _playerinfo_players_knocked_out_ra_4 _playerinfo_times_taunted_4 _playerinfo_pointsround_4 _skeletalmesh_3) Player))
    (:`0_Base2`
      (message `/Game/Data/Interact_Interface.ChangeOutfit` Player _skeletalmesh_4)
      (set `/Game/Blueprints/Characters/Golem/0_Base.PlayerInfo` (make `/Game/Blueprints/Characters/Golem/Struct_PlayerInfo` _playerinfo_playername_3 _playerinfo_rank_3 _playerinfo_items_crafted_3 _playerinfo_products_shipped_3 _playerinfo_tasks_completed_3 _playerinfo_players_knocked_out_3 _playerinfo_players_knocked_out_unarmed_3 _playerinfo_players_knocked_out_1h_3 _playerinfo_players_knocked_out_2h_3 _playerinfo_players_knocked_out_sp_3 _playerinfo_players_knocked_out_ra_3 _playerinfo_times_taunted_3 _playerinfo_pointsround_3 _skeletalmesh_4) Player))
    (:`0_Base3`
      (message `/Game/Data/Interact_Interface.ChangeOutfit` Player _skeletalmesh)
      (set `/Game/Blueprints/Characters/Golem/0_Base.PlayerInfo` (make `/Game/Blueprints/Characters/Golem/Struct_PlayerInfo` _playerinfo_playername _playerinfo_rank _playerinfo_items_crafted _playerinfo_products_shipped _playerinfo_tasks_completed _playerinfo_players_knocked_out _playerinfo_players_knocked_out_unarmed _playerinfo_players_knocked_out_1h _playerinfo_players_knocked_out_2h _playerinfo_players_knocked_out_sp _playerinfo_players_knocked_out_ra _playerinfo_times_taunted _playerinfo_pointsround _skeletalmesh) Player))))

(event `/Game/Data/Interact_Interface.CycleMenu`
  (params (Right :type Boolean) (Player :type "/Game/Blueprints/Characters/Golem/0_Base Object Reference"))
  (switch `string` (`KismetSystemLibrary.GetDisplayName` Player)
    (:`0_Base`
      (`self.Player1Handling` Player Right))
    (:`0_Base1`
      (`self.Player2Handling` Player Right))
    (:`0_Base2`
      (`self.Player3Handling` Player Right))
    (:`0_Base3`
      (`self.Player4Handling` Player Right))))

(event `/Game/Data/Interact_Interface.Interact`
  (params (Player :type "/Game/Blueprints/Characters/Golem/0_Base Object Reference"))
  (message `/Game/Data/Interact_Interface.OpenLocker` Player Player self)
  (`KismetArrayLibrary.Array_Add` (`self.ArrayOfPlayers`) Player)
  (bind _returnvalue (`|CreateWidget` "/Game/Blueprints/Environment/Locker/WBP_Locker.WBP_Locker_C"))
  (`KismetArrayLibrary.Array_Add` (`self.ArrayOfHUDs`) _returnvalue)
  (`UserWidget.AddToViewport` _returnvalue 0)
  (bind _returnvalue_2 (`WidgetLayoutLibrary.SlotAsCanvasSlot` (`/Game/Blueprints/Environment/Locker/WBP_Locker.Border_128` _returnvalue)))
  (`KismetArrayLibrary.Array_Add` (`self.ArrayOfHUDSlots`) _returnvalue_2)
  (for (_array_element _array_index) (`self.ArrayOfOutfits`)
    (if (== _array_element (`SkinnedMeshComponent.SkeletalMesh` (`Character.Mesh` Player)))
      (switch `string` (`KismetSystemLibrary.GetDisplayName` Player)
        (:`0_Base`
          (set `self.CurrentItemIndex0` _array_index)
          (bind _output (`|GetArrayItem` (`self.ArrayOfOutfits`) _array_index))
          (`/Game/Blueprints/Environment/Locker/BP_HudCharacter.SetPreviewMesh` (`self.HudCharacter0`) _output)
          (set `self.HUDMinAnchors` (0.0 0.0))
          (set `self.HUDMaxAnchors` (0.0 0.0))
          (set `self.HUDXPos` 50.0)
          (set `self.HUDYPos` 50.0)
          (bind _characterpreview (`/Game/Blueprints/Environment/Locker/WBP_Locker.CharacterPreview` _returnvalue))
          (`Image.SetBrushFromMaterial` _characterpreview "/Game/Blueprints/Environment/Locker/mat_HUDCharacter.mat_HUDCharacter"))
        (:`0_Base1`
          (set `self.CurrentItemIndex1` _array_index)
          (`/Game/Blueprints/Environment/Locker/BP_HudCharacter.SetPreviewMesh` (`self.HudCharacter1`) _output)
          (set `self.HUDMinAnchors` (1.0 0.0))
          (set `self.HUDMaxAnchors` (1.0 0.0))
          (set `self.HUDXPos` -550.0)
          (set `self.HUDYPos` 50.0)
          (`Image.SetBrushFromMaterial` _characterpreview "/Game/Blueprints/Environment/Locker/mat_HUDCharacter_Inst1.mat_HUDCharacter_Inst1"))
        (:`0_Base2`
          (set `self.CurrentItemIndex2` _array_index)
          (`/Game/Blueprints/Environment/Locker/BP_HudCharacter.SetPreviewMesh` (`self.HudCharacter2`) _output)
          (set `self.HUDMinAnchors` (0.0 1.0))
          (set `self.HUDMaxAnchors` (0.0 1.0))
          (set `self.HUDXPos` 50.0)
          (set `self.HUDYPos` -550.0)
          (`Image.SetBrushFromMaterial` _characterpreview "/Game/Blueprints/Environment/Locker/mat_HUDCharacter_Inst2.mat_HUDCharacter_Inst2"))
        (:`0_Base3`
          (set `self.CurrentItemIndex3` _array_index)
          (`/Game/Blueprints/Environment/Locker/BP_HudCharacter.SetPreviewMesh` (`self.HudCharacter3`) _output)
          (set `self.HUDMinAnchors` (1.0 1.0))
          (set `self.HUDMaxAnchors` (1.0 1.0))
          (set `self.HUDXPos` -550.0)
          (set `self.HUDYPos` -550.0)
          (`Image.SetBrushFromMaterial` _characterpreview "/Game/Blueprints/Environment/Locker/mat_HUDCharacter_Inst3.mat_HUDCharacter_Inst3")))
      (`CanvasPanelSlot.SetAnchors` _returnvalue_2 (make `Anchors` (`self.HUDMinAnchors`) (`self.HUDMaxAnchors`)))
      (`CanvasPanelSlot.SetPosition` _returnvalue_2 (`KismetMathLibrary.MakeVector2D` (`self.HUDXPos`) (`self.HUDYPos`))))))

(event `self.InteractArea.OnComponentEndOverlap`
  (params (OverlappedComponent :type "PrimitiveComponent Object Reference") (OtherActor :type "Actor Object Reference") (OtherComp :type "PrimitiveComponent Object Reference") (OtherBodyIndex :type Integer))
  (bind _arrayofhuds (`self.ArrayOfHUDs`))
  ;[1 1 1] Close UI
  (bind _as0_base (cast `/Game/Blueprints/Characters/Golem/0_Base` OtherActor))
  (set `/Game/Blueprints/Characters/Golem/0_Base.Locker` null _as0_base)
  (for (_array_element _array_index) (`self.ArrayOfPlayers`)
    (if (`KismetStringLibrary.EqualEqual_StrStr` (`KismetSystemLibrary.GetDisplayName` _array_element) (`KismetSystemLibrary.GetDisplayName` _as0_base))
      (`KismetArrayLibrary.Array_Remove` (`self.ArrayOfPlayers`) _array_index)
      (`Widget.RemoveFromParent` (`|GetArrayItem` _arrayofhuds _array_index))
      (`KismetArrayLibrary.Array_Remove` _arrayofhuds _array_index)
      (`KismetArrayLibrary.Array_Remove` (`self.ArrayOfHUDSlots`) _array_index)
      (switch `string` (`KismetSystemLibrary.GetDisplayName` _as0_base)
        (:`0_Base`
          (set `self.P1Int` 0))
        (:`0_Base1`
          (set `self.P2Int` 0))
        (:`0_Base2`
          (set `self.P3Int` 0))
        (:`0_Base3`
          (set `self.P4Int` 0))))))

(fn `CheckP1Outfit`
  (params (Player :type "/Game/Blueprints/Characters/Golem/0_Base Object Reference") (Right :type Boolean))
  (for (_array_element _array_index) (`self.ArrayOfOutfits`)
    (if (`KismetStringLibrary.EqualEqual_StrStr` (`KismetSystemLibrary.GetDisplayName` _array_element) (`KismetSystemLibrary.GetDisplayName` (`SkinnedMeshComponent.SkeletalMesh` (`Character.Mesh` Player))))
      (if Right
        (if (== (`self.CurrentItemIndex0`) (- (`KismetArrayLibrary.Array_Length` (`self.ArrayOfOutfits`)) 1))
          (bind _output_get (set `self.CurrentItemIndex0` 0))
          (`/Game/Blueprints/Environment/Locker/BP_HudCharacter.SetPreviewMesh` (`self.HudCharacter0`) (`|GetArrayItem` (`self.ArrayOfOutfits`) _output_get))
          (else
            (bind _output_get_2 (set `self.CurrentItemIndex0` _array_index))
            (bind _result (`/Engine/EditorBlueprintResources/StandardMacros.IncrementInt` _output_get_2)
              (:`  `
                (`/Game/Blueprints/Environment/Locker/BP_HudCharacter.SetPreviewMesh` (`self.HudCharacter0`) (`|GetArrayItem` (`self.ArrayOfOutfits`) _result))))))
        (elif (== (`self.CurrentItemIndex0`) 0)
          (bind _output_get_3 (set `self.CurrentItemIndex0` (- (`KismetArrayLibrary.Array_Length` (`self.ArrayOfOutfits`)) 1)))
          (`/Game/Blueprints/Environment/Locker/BP_HudCharacter.SetPreviewMesh` (`self.HudCharacter0`) (`|GetArrayItem` (`self.ArrayOfOutfits`) _output_get_3))
          (else
            (bind _output_get_4 (set `self.CurrentItemIndex0` _array_index))
            (bind _result_2 (`/Engine/EditorBlueprintResources/StandardMacros.DecrementInt` _output_get_4)
              (:`  `
                (`/Game/Blueprints/Environment/Locker/BP_HudCharacter.SetPreviewMesh` (`self.HudCharacter0`) (`|GetArrayItem` (`self.ArrayOfOutfits`) _result_2))))))))))

(fn `CheckP2Outfit`
  (params (Player :type "/Game/Blueprints/Characters/Golem/0_Base Object Reference") (Right :type Boolean))
  (for (_array_element _array_index) (`self.ArrayOfOutfits`)
    (if (`KismetStringLibrary.EqualEqual_StrStr` (`KismetSystemLibrary.GetDisplayName` _array_element) (`KismetSystemLibrary.GetDisplayName` (`SkinnedMeshComponent.SkeletalMesh` (`Character.Mesh` Player))))
      (if Right
        (if (== (`self.CurrentItemIndex1`) (- (`KismetArrayLibrary.Array_Length` (`self.ArrayOfOutfits`)) 1))
          (bind _output_get (set `self.CurrentItemIndex1` 0))
          (`/Game/Blueprints/Environment/Locker/BP_HudCharacter.SetPreviewMesh` (`self.HudCharacter1`) (`|GetArrayItem` (`self.ArrayOfOutfits`) _output_get))
          (else
            (bind _output_get_2 (set `self.CurrentItemIndex1` _array_index))
            (bind _result (`/Engine/EditorBlueprintResources/StandardMacros.IncrementInt` _output_get_2)
              (:`  `
                (`/Game/Blueprints/Environment/Locker/BP_HudCharacter.SetPreviewMesh` (`self.HudCharacter1`) (`|GetArrayItem` (`self.ArrayOfOutfits`) _result))))))
        (elif (== (`self.CurrentItemIndex1`) 0)
          (bind _output_get_3 (set `self.CurrentItemIndex1` (- (`KismetArrayLibrary.Array_Length` (`self.ArrayOfOutfits`)) 1)))
          (`/Game/Blueprints/Environment/Locker/BP_HudCharacter.SetPreviewMesh` (`self.HudCharacter1`) (`|GetArrayItem` (`self.ArrayOfOutfits`) _output_get_3))
          (else
            (bind _output_get_4 (set `self.CurrentItemIndex1` _array_index))
            (bind _result_2 (`/Engine/EditorBlueprintResources/StandardMacros.DecrementInt` _output_get_4)
              (:`  `
                (`/Game/Blueprints/Environment/Locker/BP_HudCharacter.SetPreviewMesh` (`self.HudCharacter1`) (`|GetArrayItem` (`self.ArrayOfOutfits`) _result_2))))))))))

(fn `CheckP3Outfit`
  (params (Player :type "/Game/Blueprints/Characters/Golem/0_Base Object Reference") (Right :type Boolean))
  (for (_array_element _array_index) (`self.ArrayOfOutfits`)
    (if (`KismetStringLibrary.EqualEqual_StrStr` (`KismetSystemLibrary.GetDisplayName` _array_element) (`KismetSystemLibrary.GetDisplayName` (`SkinnedMeshComponent.SkeletalMesh` (`Character.Mesh` Player))))
      (if Right
        (if (== (`self.CurrentItemIndex2`) (- (`KismetArrayLibrary.Array_Length` (`self.ArrayOfOutfits`)) 1))
          (bind _output_get (set `self.CurrentItemIndex2` 0))
          (`/Game/Blueprints/Environment/Locker/BP_HudCharacter.SetPreviewMesh` (`self.HudCharacter2`) (`|GetArrayItem` (`self.ArrayOfOutfits`) _output_get))
          (else
            (bind _output_get_2 (set `self.CurrentItemIndex2` _array_index))
            (bind _result (`/Engine/EditorBlueprintResources/StandardMacros.IncrementInt` _output_get_2)
              (:`  `
                (`/Game/Blueprints/Environment/Locker/BP_HudCharacter.SetPreviewMesh` (`self.HudCharacter2`) (`|GetArrayItem` (`self.ArrayOfOutfits`) _result))))))
        (elif (== (`self.CurrentItemIndex2`) 0)
          (bind _output_get_3 (set `self.CurrentItemIndex2` (- (`KismetArrayLibrary.Array_Length` (`self.ArrayOfOutfits`)) 1)))
          (`/Game/Blueprints/Environment/Locker/BP_HudCharacter.SetPreviewMesh` (`self.HudCharacter2`) (`|GetArrayItem` (`self.ArrayOfOutfits`) _output_get_3))
          (else
            (bind _output_get_4 (set `self.CurrentItemIndex2` _array_index))
            (bind _result_2 (`/Engine/EditorBlueprintResources/StandardMacros.DecrementInt` _output_get_4)
              (:`  `
                (`/Game/Blueprints/Environment/Locker/BP_HudCharacter.SetPreviewMesh` (`self.HudCharacter2`) (`|GetArrayItem` (`self.ArrayOfOutfits`) _result_2))))))))))

(fn `CheckP4Outfit`
  (params (Player :type "/Game/Blueprints/Characters/Golem/0_Base Object Reference") (Right :type Boolean))
  (for (_array_element _array_index) (`self.ArrayOfOutfits`)
    (if (`KismetStringLibrary.EqualEqual_StrStr` (`KismetSystemLibrary.GetDisplayName` _array_element) (`KismetSystemLibrary.GetDisplayName` (`SkinnedMeshComponent.SkeletalMesh` (`Character.Mesh` Player))))
      (if Right
        (if (== (`self.CurrentItemIndex3`) (- (`KismetArrayLibrary.Array_Length` (`self.ArrayOfOutfits`)) 1))
          (bind _output_get (set `self.CurrentItemIndex3` 0))
          (`/Game/Blueprints/Environment/Locker/BP_HudCharacter.SetPreviewMesh` (`self.HudCharacter3`) (`|GetArrayItem` (`self.ArrayOfOutfits`) _output_get))
          (else
            (bind _output_get_2 (set `self.CurrentItemIndex3` _array_index))
            (bind _result (`/Engine/EditorBlueprintResources/StandardMacros.IncrementInt` _output_get_2)
              (:`  `
                (`/Game/Blueprints/Environment/Locker/BP_HudCharacter.SetPreviewMesh` (`self.HudCharacter3`) (`|GetArrayItem` (`self.ArrayOfOutfits`) _result))))))
        (elif (== (`self.CurrentItemIndex3`) 0)
          (bind _output_get_3 (set `self.CurrentItemIndex3` (- (`KismetArrayLibrary.Array_Length` (`self.ArrayOfOutfits`)) 1)))
          (`/Game/Blueprints/Environment/Locker/BP_HudCharacter.SetPreviewMesh` (`self.HudCharacter3`) (`|GetArrayItem` (`self.ArrayOfOutfits`) _output_get_3))
          (else
            (bind _output_get_4 (set `self.CurrentItemIndex3` _array_index))
            (bind _result_2 (`/Engine/EditorBlueprintResources/StandardMacros.DecrementInt` _output_get_4)
              (:`  `
                (`/Game/Blueprints/Environment/Locker/BP_HudCharacter.SetPreviewMesh` (`self.HudCharacter3`) (`|GetArrayItem` (`self.ArrayOfOutfits`) _result_2))))))))))

(fn `P1CycleLeft`
  (bind _currentitemindex0 (`self.CurrentItemIndex0`))
  (if (== (`self.CurrentItemIndex0`) 0)
    (set `self.CurrentItemIndex0` (- (`KismetArrayLibrary.Array_Length` (`self.ArrayOfOutfits`)) 1))
    (else
      (`/Engine/EditorBlueprintResources/StandardMacros.DecrementInt` _currentitemindex0
        (:`  `
          _))))
  (`/Game/Blueprints/Environment/Locker/BP_HudCharacter.SetPreviewMesh` (`self.HudCharacter0`) (`|GetArrayItem` (`self.ArrayOfOutfits`) _currentitemindex0)))

(fn `P1CycleRight`
  (bind _currentitemindex0 (`self.CurrentItemIndex0`))
  (if (== (`self.CurrentItemIndex0`) (- (`KismetArrayLibrary.Array_Length` (`self.ArrayOfOutfits`)) 1))
    (set `self.CurrentItemIndex0` 0)
    (else
      (`/Engine/EditorBlueprintResources/StandardMacros.IncrementInt` _currentitemindex0
        (:`  `
          _))))
  (`/Game/Blueprints/Environment/Locker/BP_HudCharacter.SetPreviewMesh` (`self.HudCharacter0`) (`|GetArrayItem` (`self.ArrayOfOutfits`) _currentitemindex0)))

(fn `P2CycleLeft`
  (bind _currentitemindex1 (`self.CurrentItemIndex1`))
  (if (== (`self.CurrentItemIndex1`) 0)
    (set `self.CurrentItemIndex1` (- (`KismetArrayLibrary.Array_Length` (`self.ArrayOfOutfits`)) 1))
    (else
      (`/Engine/EditorBlueprintResources/StandardMacros.DecrementInt` _currentitemindex1
        (:`  `
          _))))
  (`/Game/Blueprints/Environment/Locker/BP_HudCharacter.SetPreviewMesh` (`self.HudCharacter1`) (`|GetArrayItem` (`self.ArrayOfOutfits`) _currentitemindex1)))

(fn `P2CycleRight`
  (bind _currentitemindex1 (`self.CurrentItemIndex1`))
  (if (== (`self.CurrentItemIndex1`) (- (`KismetArrayLibrary.Array_Length` (`self.ArrayOfOutfits`)) 1))
    (set `self.CurrentItemIndex1` 0)
    (else
      (`/Engine/EditorBlueprintResources/StandardMacros.IncrementInt` _currentitemindex1
        (:`  `
          _))))
  (`/Game/Blueprints/Environment/Locker/BP_HudCharacter.SetPreviewMesh` (`self.HudCharacter1`) (`|GetArrayItem` (`self.ArrayOfOutfits`) _currentitemindex1)))

(fn `P3CycleLeft`
  (bind _currentitemindex2 (`self.CurrentItemIndex2`))
  (if (== (`self.CurrentItemIndex2`) 0)
    (set `self.CurrentItemIndex2` (- (`KismetArrayLibrary.Array_Length` (`self.ArrayOfOutfits`)) 1))
    (else
      (`/Engine/EditorBlueprintResources/StandardMacros.DecrementInt` _currentitemindex2
        (:`  `
          _))))
  (`/Game/Blueprints/Environment/Locker/BP_HudCharacter.SetPreviewMesh` (`self.HudCharacter2`) (`|GetArrayItem` (`self.ArrayOfOutfits`) _currentitemindex2)))

(fn `P3CycleRight`
  (bind _currentitemindex2 (`self.CurrentItemIndex2`))
  (if (== (`self.CurrentItemIndex2`) (- (`KismetArrayLibrary.Array_Length` (`self.ArrayOfOutfits`)) 1))
    (set `self.CurrentItemIndex2` 0)
    (else
      (`/Engine/EditorBlueprintResources/StandardMacros.IncrementInt` _currentitemindex2
        (:`  `
          _))))
  (`/Game/Blueprints/Environment/Locker/BP_HudCharacter.SetPreviewMesh` (`self.HudCharacter2`) (`|GetArrayItem` (`self.ArrayOfOutfits`) _currentitemindex2)))

(fn `P4CycleLeft`
  (bind _currentitemindex3 (`self.CurrentItemIndex3`))
  (if (== (`self.CurrentItemIndex3`) 0)
    (set `self.CurrentItemIndex3` (- (`KismetArrayLibrary.Array_Length` (`self.ArrayOfOutfits`)) 1))
    (else
      (`/Engine/EditorBlueprintResources/StandardMacros.DecrementInt` _currentitemindex3
        (:`  `
          _))))
  (`/Game/Blueprints/Environment/Locker/BP_HudCharacter.SetPreviewMesh` (`self.HudCharacter3`) (`|GetArrayItem` (`self.ArrayOfOutfits`) _currentitemindex3)))

(fn `P4CycleRight`
  (bind _currentitemindex3 (`self.CurrentItemIndex3`))
  (if (== (`self.CurrentItemIndex3`) (- (`KismetArrayLibrary.Array_Length` (`self.ArrayOfOutfits`)) 1))
    (set `self.CurrentItemIndex3` 0)
    (else
      (`/Engine/EditorBlueprintResources/StandardMacros.IncrementInt` _currentitemindex3
        (:`  `
          _))))
  (`/Game/Blueprints/Environment/Locker/BP_HudCharacter.SetPreviewMesh` (`self.HudCharacter3`) (`|GetArrayItem` (`self.ArrayOfOutfits`) _currentitemindex3)))

(fn `Player1Handling`
  (params (Player :type "/Game/Blueprints/Characters/Golem/0_Base Object Reference") (Right :type Boolean))
  (switch `int` (`self.P1Int`)
    (:`0`
      (`self.CheckP1Outfit` Player Right)
      (set `self.P1Int` 1))
    (:`1`
      (if Right
        (`self.P1CycleRight`)
        (else
          (`self.P1CycleLeft`))))))

(fn `Player2Handling`
  (params (Player :type "/Game/Blueprints/Characters/Golem/0_Base Object Reference") (Right :type Boolean))
  (switch `int` (`self.P2Int`)
    (:`0`
      (`self.CheckP2Outfit` Player Right)
      (set `self.P2Int` 1))
    (:`1`
      (if Right
        (`self.P2CycleRight`)
        (else
          (`self.P2CycleLeft`))))))

(fn `Player3Handling`
  (params (Player :type "/Game/Blueprints/Characters/Golem/0_Base Object Reference") (Right :type Boolean))
  (switch `int` (`self.P3Int`)
    (:`0`
      (`self.CheckP3Outfit` Player Right)
      (set `self.P3Int` 1))
    (:`1`
      (if Right
        (`self.P3CycleRight`)
        (else
          (`self.P3CycleLeft`))))))

(fn `Player4Handling`
  (params (Player :type "/Game/Blueprints/Characters/Golem/0_Base Object Reference") (Right :type Boolean))
  (switch `int` (`self.P4Int`)
    (:`0`
      (`self.CheckP4Outfit` Player Right)
      (set `self.P4Int` 1))
    (:`1`
      (if Right
        (`self.P4CycleRight`)
        (else
          (`self.P4CycleLeft`))))))

(fn `UserConstructionScript`)