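; Spline-based conveyor belt that carries overlapping objects along its path and can be halted by sabotage.
; The construction script places belt meshes, seven rollers and an overlap component at each spacing step along the spline.
; A looping timer nudges overlapping actors of listed classes along the nearest spline direction, filtering by attach parent and moving each once per pass.
; Tick spins the rollers; Sabotage and StopSabotage pause or resume both motions.
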(event `self.ReceiveBeginPlay`
  ;[1 1 1] Move Objects
  (bind _outactors (`GameplayStatics.GetAllActorsOfClass` "/Game/Blueprints/Environment/Conveyor/BP_SabotageMachine.BP_SabotageMachine_C"))
  (set `self.SabotageMachines` _outactors)
  (bind _returnvalue (`KismetSystemLibrary.K2_SetTimerDelegate` (delegate `MoveObjects`) 0.01 true))
  (set `self.MoveTimerHandle` _returnvalue))

(event `MoveObjects`
  (bind (_returnvalue_roll _returnvalue_pitch _returnvalue_yaw) (`KismetMathLibrary.BreakRotator` (`SceneComponent.K2_GetComponentRotation` (`self.DefaultSceneRoot`))))
  ;[1 1 1] Move Objects
  (set `self.MovedActors` (`|MakeArray` self :!type "Actor Object Reference"))
  (for _array_element (`self.OverlapComponent`)
    (for _array_element_2 (`self.ClassArray`)
      (for _array_element_3 (`PrimitiveComponent.GetOverlappingActors` _array_element _array_element_2)
        (if (== (`KismetArrayLibrary.Array_Find` (`self.MovedActors`) _array_element_3) -1)
          (if (== (`self.GetAttachParentActor` _array_element_3) null)
            (`self.K2_AddActorWorldOffset` _array_element_3 (`KismetMathLibrary.GreaterGreater_VectorRotator` (* (`SplineComponent.FindDirectionClosestToWorldLocation` (`self.Spline`) (`self.K2_GetActorLocation` _array_element_3) "Local") (`self.DynamicSpeed`)) (`KismetMathLibrary.MakeRotator` _returnvalue_roll _returnvalue_pitch (- _returnvalue_yaw 270.0))) false false)
            (`KismetArrayLibrary.Array_Add` (`self.MovedActors`) _array_element_3)))))))

(event `Sabotage`
  ;[1 1 1] Sabotage
  (set `self.Sabotaged` false)
  (`KismetSystemLibrary.K2_PauseTimerHandle` (`self.MoveTimerHandle`))
  (set `self.RollerSpeed` 0.0))

(event `self.ReceiveTick`
  (params (DeltaSeconds :type "Float (single-precision)"))
  ;[1 1 1] Animation for Rollers
  (for _array_element (`self.Roller`)
    (`SceneComponent.K2_AddLocalRotation` _array_element (`KismetMathLibrary.MakeRotator` (`self.RollerSpeed`)) false false)))

(event `StopSabotage`
  ;[1 1 1] Sabotage
  (set `self.Sabotaged` true)
  (`KismetSystemLibrary.K2_UnPauseTimerHandle` (`self.MoveTimerHandle`))
  (set `self.RollerSpeed` 2.0))

(event `SetPlayer`
  (params (Player :type "/Game/Blueprints/Characters/Golem/0_Base Object Reference"))
  ;[1 1 1] Set Player
  (set `self.Player` Player))

(fn `UserConstructionScript`
  (for _index (range (+ (`KismetMathLibrary.FFloor` (/ (`SplineComponent.GetSplineLength` (`self.Spline`)) (`self.Spacing`))) 1))
    (bind _returnvalue (`KismetMathLibrary.InverseTransformLocation` (`self.GetTransform`) (`SplineComponent.GetLocationAtDistanceAlongSpline` (`self.Spline`) (* _index (`self.Spacing`)) "World")))
    (bind _returnvalue_2 (`AddComponent|NODE_AddSplineMeshComponent-5` :`RelativeTransform` (`KismetMathLibrary.MakeTransform` (+ _returnvalue (0.0 0.0 -50.0)) (struct) (1.18 1.0 1.0))))
    (`KismetArrayLibrary.Array_Add` (`self.MeshComponent`) _returnvalue_2)
    (bind _returnvalue_3 (`AddComponent|NODE_AddSplineMeshComponent-16` :`RelativeTransform` (`KismetMathLibrary.MakeTransform` (+ _returnvalue (`|GetArrayItem` (`self.RollerLocation`))))))
    (`KismetArrayLibrary.Array_Add` (`self.Roller`) _returnvalue_3)
    (bind _returnvalue_4 (`AddComponent|NODE_AddSplineMeshComponent-19` :`RelativeTransform` (`KismetMathLibrary.MakeTransform` (+ _returnvalue (`|GetArrayItem` (`self.RollerLocation`) 1)))))
    (`KismetArrayLibrary.Array_Add` (`self.Roller`) _returnvalue_4)
    (bind _returnvalue_5 (`AddComponent|NODE_AddSplineMeshComponent-20` :`RelativeTransform` (`KismetMathLibrary.MakeTransform` (+ _returnvalue (`|GetArrayItem` (`self.RollerLocation`) 2)))))
    (`KismetArrayLibrary.Array_Add` (`self.Roller`) _returnvalue_5)
    (bind _returnvalue_6 (`AddComponent|NODE_AddSplineMeshComponent-21` :`RelativeTransform` (`KismetMathLibrary.MakeTransform` (+ _returnvalue (`|GetArrayItem` (`self.RollerLocation`) 3)))))
    (`KismetArrayLibrary.Array_Add` (`self.Roller`) _returnvalue_6)
    (bind _returnvalue_7 (`AddComponent|NODE_AddSplineMeshComponent-22` :`RelativeTransform` (`KismetMathLibrary.MakeTransform` (+ _returnvalue (`|GetArrayItem` (`self.RollerLocation`) 4)))))
    (`KismetArrayLibrary.Array_Add` (`self.Roller`) _returnvalue_7)
    (bind _returnvalue_8 (`AddComponent|NODE_AddSplineMeshComponent-23` :`RelativeTransform` (`KismetMathLibrary.MakeTransform` (+ _returnvalue (`|GetArrayItem` (`self.RollerLocation`) 5)))))
    (`KismetArrayLibrary.Array_Add` (`self.Roller`) _returnvalue_8)
    (bind _returnvalue_9 (`AddComponent|NODE_AddSplineMeshComponent-24` :`RelativeTransform` (`KismetMathLibrary.MakeTransform` (+ _returnvalue (`|GetArrayItem` (`self.RollerLocation`) 6)))))
    (`KismetArrayLibrary.Array_Add` (`self.Roller`) _returnvalue_9)
    (bind _returnvalue_10 (`AddComponent|NODE_AddSplineMeshComponent-8` :`RelativeTransform` (`KismetMathLibrary.MakeTransform` (+ _returnvalue (0.0 0.0 -40.0)) (struct) (1.18 1.0 1.0))))
    (`KismetArrayLibrary.Array_Add` (`self.OverlapComponent`) _returnvalue_10)))