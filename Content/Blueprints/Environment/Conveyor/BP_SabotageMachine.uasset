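; Sabotage machine that lets a player hold interact inside its box to disrupt the nearest conveyor.
; A timeline drives the progress widget and looping-once fix sound, resetting if the player releases or leaves.
; On completion it branches on the conveyor's Sabotaged flag: true triggers sabotage, steam, 4 round points and a scoreboard update, then reverts after 30 seconds.
; False stops the sabotage and steam immediately.
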(event `self.ReceiveBeginPlay`
  (bind _asbp_sabotage_widget (cast `/Game/Blueprints/Environment/Conveyor/BP_SabotageWidget` (`WidgetComponent.GetUserWidgetObject` (`self.SabotageWidget`))))
  (set `self.ProgressWidget` _asbp_sabotage_widget))

(event `/Game/Data/Interact_Interface.Interact`
  (params (Player :type "/Game/Blueprints/Characters/Golem/0_Base Object Reference"))
  (bind _p_steam (`self.P_Steam`))
  (bind _sabotaged (`/Game/Blueprints/Environment/Conveyor/BP_ConveyorSpawner.Sabotaged` (`self.NearestConveyor`)))
  (set `self.Player` Player)
  (`TimelineComponent.SetNewTime` (`self.SabotagePercentage`) 0.0)
  (bind (_direction _0_1) (`Timeline|SabotagePercentage`)
    (:`Update`
      (if (`/Game/Blueprints/Characters/Golem/0_Base.IsInteracting` (`self.Player`))
        (if (`PrimitiveComponent.IsOverlappingActor` (`self.Box`) (`self.Player`))
          (`/Game/Blueprints/Environment/Conveyor/BP_SabotageWidget.SetProgress` (`self.ProgressWidget`) _0_1)
          (`/Engine/EditorBlueprintResources/StandardMacros.DoOnce` false :!label _label
            (:`Completed`
              (bind _returnvalue (`GameplayStatics.SpawnSoundAttached` "/Game/Audio/SFX/SE_ToolsFixing.SE_ToolsFixing" (`self.SabotageMachine`) "None" (0.0 0.0 0.0) (struct) "KeepRelativeOffset" false 0.5 1.0 0.0 null null))))
          (else
            (`TimelineComponent.Stop` (`self.SabotagePercentage`) :!label _label_2)
            (`/Game/Blueprints/Environment/Conveyor/BP_SabotageWidget.SetProgress` (`self.ProgressWidget`) 0.0)
            (`/Engine/EditorBlueprintResources/StandardMacros.IsValid` _returnvalue :!label _label_3
              (:`Is Valid`
                (`AudioComponent.Stop` _returnvalue)
                (goto _label :!via `Reset`)))))
        (else
          (goto _label_2))))
    (:`Finished`
      (`KismetSystemLibrary.PrintString` (`KismetStringLibrary.Conv_BoolToString` _sabotaged))
      (if _sabotaged
        (`/Game/Blueprints/Environment/Conveyor/BP_SabotageWidget.SetProgress` (`self.ProgressWidget`) 0.0)
        (`ActorComponent.Activate` _p_steam false)
        (`/Game/Blueprints/Environment/Conveyor/BP_ConveyorSpawner.Sabotage` (`self.NearestConveyor`))
        (bind _as0_base (cast `/Game/Blueprints/Characters/Golem/0_Base` (`self.Player`)))
        (bind (_playerinfo_playername _playerinfo_rank _playerinfo_items_crafted _playerinfo_products_shipped _playerinfo_tasks_completed _playerinfo_players_knocked_out _playerinfo_players_knocked_out_unarmed _playerinfo_players_knocked_out_1h _playerinfo_players_knocked_out_2h _playerinfo_players_knocked_out_sp _playerinfo_players_knocked_out_ra _playerinfo_times_taunted _playerinfo_pointsround _playerinfo_outfit) (break `/Game/Blueprints/Characters/Golem/Struct_PlayerInfo` (`/Game/Blueprints/Characters/Golem/0_Base.PlayerInfo` _as0_base)))
        (set `/Game/Blueprints/Characters/Golem/0_Base.PlayerInfo` (make `/Game/Blueprints/Characters/Golem/Struct_PlayerInfo` _playerinfo_playername _playerinfo_rank _playerinfo_items_crafted _playerinfo_products_shipped _playerinfo_tasks_completed _playerinfo_players_knocked_out _playerinfo_players_knocked_out_unarmed _playerinfo_players_knocked_out_1h _playerinfo_players_knocked_out_2h _playerinfo_players_knocked_out_sp _playerinfo_players_knocked_out_ra _playerinfo_times_taunted (+ _playerinfo_pointsround 4) _playerinfo_outfit) _as0_base)
        (message `/Game/Data/Interact_Interface.UpdateScore` (`/Game/Blueprints/Characters/Golem/0_Base.Scoreboard` _as0_base))
        (`KismetSystemLibrary.Delay` 30.0)
        (`/Game/Blueprints/Environment/Conveyor/BP_ConveyorSpawner.StopSabotage` (`self.NearestConveyor`))
        (`ActorComponent.Deactivate` _p_steam)
        (goto _label_3)
        (else
          (`/Game/Blueprints/Environment/Conveyor/BP_SabotageWidget.SetProgress` (`self.ProgressWidget`) 0.0)
          (`/Game/Blueprints/Environment/Conveyor/BP_ConveyorSpawner.StopSabotage` (`self.NearestConveyor`))
          (`ActorComponent.Deactivate` (`self.P_Steam`)))))))

(fn `UserConstructionScript`)