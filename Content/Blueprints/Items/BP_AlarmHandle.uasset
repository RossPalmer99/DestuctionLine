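; BP_AlarmHandle is a handle item that combines with a BP_AlarmClock to form a weapon for the player.
; The first overlapping clock snaps to the AlarmSocket on the skeletal mesh, with physics disabled and collision responses adjusted.
; The handle copies the clock's damage, power and chip stats, sets the same ItemInfo flag on both items, then has the player select it as a weapon.
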(event `self.AlarmCollision.OnComponentBeginOverlap`
  (params (OverlappedComponent :type "PrimitiveComponent Object Reference") (OtherActor :type "Actor Object Reference") (OtherComp :type "PrimitiveComponent Object Reference") (OtherBodyIndex :type Integer) (bFromSweep :type Boolean) (SweepResult :type "HitResult Structure (by ref)"))
  (bind (_iteminfo_isproduct _iteminfo_isweapon1h _iteminfo_isweapon2h _iteminfo_isstacktruck _iteminfo_isfireextinguisher _iteminfo_isaccessory _iteminfo_ispowerup _iteminfo_isalarmclock _iteminfo_isbarrel _iteminfo_damage _iteminfo_weaponpower _iteminfo_weaponchip _iteminfo_colour _iteminfo_pointvalue _iteminfo_isstungun) (break `/Game/Blueprints/Items/Data/Struct_ItemInfo` (`self.ItemInfo`)))
  (bind _asbp_alarm_clock (cast `/Game/Blueprints/Items/BP_AlarmClock` OtherActor))
  (`/Engine/EditorBlueprintResources/StandardMacros.DoOnce` false
    (:`Completed`
      (`self.K2_AttachToComponent` _asbp_alarm_clock (`self.SkeletalMesh`) "AlarmSocket" "SnapToTarget" "SnapToTarget" "KeepRelative" true)
      (`PrimitiveComponent.SetCollisionResponseToChannel` (`/Game/Blueprints/Items/BP_MasterItem.StaticMesh` _asbp_alarm_clock) "ECC_Pawn" "ECR_Overlap")
      (`PrimitiveComponent.SetSimulatePhysics` (`/Game/Blueprints/Items/BP_MasterItem.StaticMesh` _asbp_alarm_clock) false)
      (bind (_iteminfo_isproduct_2 _iteminfo_isweapon1h_2 _iteminfo_isweapon2h_2 _iteminfo_isstacktruck_2 _iteminfo_isfireextinguisher_2 _iteminfo_isaccessory_2 _iteminfo_ispowerup_2 _iteminfo_isalarmclock_2 _iteminfo_isbarrel_2 _iteminfo_damage_2 _iteminfo_weaponpower_2 _iteminfo_weaponchip_2 _iteminfo_colour_2 _iteminfo_pointvalue_2 _iteminfo_isstungun_2) (break `/Game/Blueprints/Items/Data/Struct_ItemInfo` (`/Game/Blueprints/Items/BP_MasterItem.ItemInfo` _asbp_alarm_clock)))
      (set `self.ItemInfo` (make `/Game/Blueprints/Items/Data/Struct_ItemInfo` _iteminfo_isproduct _iteminfo_isweapon1h true _iteminfo_isstacktruck _iteminfo_isfireextinguisher _iteminfo_isaccessory _iteminfo_ispowerup _iteminfo_isalarmclock _iteminfo_isbarrel _iteminfo_damage_2 _iteminfo_weaponpower_2 _iteminfo_weaponchip_2 _iteminfo_colour _iteminfo_pointvalue _iteminfo_isstungun))
      (set `/Game/Blueprints/Items/BP_MasterItem.ItemInfo` (make `/Game/Blueprints/Items/Data/Struct_ItemInfo` _iteminfo_isproduct_2 _iteminfo_isweapon1h_2 true _iteminfo_isstacktruck_2 _iteminfo_isfireextinguisher_2 _iteminfo_isaccessory_2 _iteminfo_ispowerup_2 _iteminfo_isalarmclock_2 _iteminfo_isbarrel_2 _iteminfo_damage_2 _iteminfo_weaponpower_2 _iteminfo_weaponchip_2 _iteminfo_colour_2 _iteminfo_pointvalue_2 _iteminfo_isstungun_2) _asbp_alarm_clock)
      (bind _staticmesh (`/Game/Blueprints/Items/BP_MasterItem.StaticMesh` _asbp_alarm_clock))
      (`PrimitiveComponent.SetCollisionResponseToChannel` _staticmesh "ECC_Visibility" "ECR_Ignore")
      (`PrimitiveComponent.SetCollisionResponseToChannel` (`/Game/Blueprints/Items/BP_MasterItem.DamageDetectCollision` _asbp_alarm_clock) "ECC_Visibility" "ECR_Ignore")
      (`PrimitiveComponent.SetCollisionResponseToChannel` _staticmesh "ECC_PhysicsBody" "ECR_Block")
      (`PrimitiveComponent.SetCollisionResponseToChannel` _staticmesh "ECC_WorldStatic" "ECR_Block")
      (`/Game/Blueprints/Characters/Golem/0_Base.SelectWeapon` (`self.PlayerRef`) self))))

(fn `UserConstructionScript`
  (`parent.UserConstructionScript`))