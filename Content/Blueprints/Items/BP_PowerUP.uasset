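; Item Blueprint for a power-up or throwable variant, configured on BeginPlay from PowerInfo as a Points, Speed, Damage or Jump effect.
; Interacting consumes a power-up immediately, while the non-power-up variant is picked up or dropped.
; A thrown item still moving fast applies its effect to whatever it hits other than the thrower.
; Hitting a 0_Base runs a DoOnce that awards thrower points, plays feedback, then hides and destroys the item.
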(event `self.ReceiveBeginPlay`
  (bind (_powerinfo_power _powerinfo_ispowerup) (break `/Game/Blueprints/Items/Data/Struct_PowerInfo` (`self.PowerInfo`)))
  ;[1 1 1] Begin Play - Sets power
  (`parent.ReceiveBeginPlay`)
  (if (== _powerinfo_power "Points")
    (`self.SetPowerUP_Points` _powerinfo_ispowerup)
    (elif (== _powerinfo_power "Speed")
      (`self.SetPowerUP_Speed` _powerinfo_ispowerup)
      (elif (== _powerinfo_power "Damage")
        (`self.SetPowerUP_Damage` _powerinfo_ispowerup)
        (elif (== _powerinfo_power "Jump")
          (`self.SetPowerUP_Jump` _powerinfo_ispowerup))))))

(event `self.ResetDoOnce`
  (goto _label :!via `Reset`))

(event `self.Throw`
  (params (PlayerThrowing :type "/Game/Blueprints/Characters/Golem/0_Base Object Reference"))
  (bind _output_get (set `self.HasBeenThrown` true)))

(event `self.ReceiveHit`
  (params (MyComp :type "PrimitiveComponent Object Reference") (Other :type "Actor Object Reference") (OtherComp :type "PrimitiveComponent Object Reference") (bSelfMoved :type Boolean) (HitLocation :type "Vector Structure") (HitNormal :type "Vector Structure") (NormalImpulse :type "Vector Structure") (Hit :type "HitResult Structure (by ref)"))
  (if (and (stale `self.Throw` _output_get) (!= (stale `self.Throw` PlayerThrowing) Other))
    (if (!= (`self.GetVelocity` self) (0.0 0.0 0.0) :`ErrorTolerance` 200.0)
      (message `/Game/Data/Interact_Interface.PowerUp` Other self)
      (if (== (`GameplayStatics.GetObjectClass` Other) "/Game/Blueprints/Characters/Golem/0_Base.0_Base_C")
        (`/Engine/EditorBlueprintResources/StandardMacros.DoOnce` false :!label _label
          (:`Completed`
            (`self.GivePoints` 10 (stale `self.Throw` PlayerThrowing))
            (message `/Game/Data/Interact_Interface.UpdateScore` (`/Game/Blueprints/Characters/Golem/0_Base.Scoreboard` (stale `self.Throw` PlayerThrowing)))
            (`self.PlaySound`)
            (`PlayerController.K2_ClientPlayForceFeedback` (`GameplayStatics.GetPlayerController` (`/Game/Blueprints/Characters/Golem/0_Base.Index` (stale `self.Throw` PlayerThrowing))) (`/Game/Blueprints/Characters/Golem/0_Base.FF_2hHit` (stale `self.Throw` PlayerThrowing)) "None" false false false)
            (`PrimitiveComponent.SetCollisionResponseToAllChannels` (`self.DamageDetectCollision`) "ECR_Ignore")
            (`PrimitiveComponent.SetCollisionResponseToAllChannels` (`self.Widget`) "ECR_Ignore")
            (`PrimitiveComponent.SetCollisionResponseToAllChannels` (`self.Sphere`) "ECR_Ignore")
            (`PrimitiveComponent.SetCollisionResponseToAllChannels` (`self.ParticleSystem`) "ECR_Ignore")
            (`PrimitiveComponent.SetCollisionResponseToAllChannels` (`self.GlowMesh`) "ECR_Ignore")
            (`PrimitiveComponent.SetCollisionResponseToAllChannels` (`self.Destructible`) "ECR_Ignore")
            (`PrimitiveComponent.SetCollisionResponseToAllChannels` (`self.StaticMesh`) "ECR_Ignore")
            (`SceneComponent.SetVisibility` (`self.StaticMesh`) false false)
            (`KismetSystemLibrary.Delay` 2.0)
            (`self.K2_DestroyActor`))))
      (else
        (set `self.HasBeenThrown` false)))))

(event `/Game/Data/Interact_Interface.Interact`
  (params (Player :type "/Game/Blueprints/Characters/Golem/0_Base Object Reference"))
  ;[1 1 1] Interact Handler
  (if (`.IsPowerUP_1_5208E18A4FDE4642235508B321CCA0FF` (break `/Game/Blueprints/Items/Data/Struct_PowerInfo` (`self.PowerInfo`)))
    (message `/Game/Data/Interact_Interface.PowerUp` Player self)
    (message `/Game/Data/Interact_Interface.Drop` self Player self)
    (`self.K2_DestroyActor`)
    (else
      (`/Engine/EditorBlueprintResources/StandardMacros.IsValid` (`/Game/Blueprints/Characters/Golem/0_Base.HeldItem` Player)
        (:`Is Valid`
          (message `/Game/Data/Interact_Interface.Drop` self Player self))
        (:`Is Not Valid`
          (`self.PlayerRef`
            (:`then`)
            (:`else`
              (message `/Game/Data/Interact_Interface.PickUp` self Player self))))))))

(fn `UserConstructionScript`
  (`parent.UserConstructionScript`))