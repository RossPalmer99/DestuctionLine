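; Stun gun projectile that electrocutes the character it hits and rewards the shooter with points.
; A sphere overlap ignores the owner, calls Electrocute on any other 0_Base actor and destroys the projectile.
; It then adds a fixed bonus to the owner's Pointsround by rebuilding its PlayerInfo struct.
; Overlaps with other actor types are ignored, and a BeginPlay delay destroys projectiles that hit nothing.
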(event `self.ReceiveBeginPlay`
  (`KismetSystemLibrary.Delay` 5.0)
  (`self.K2_DestroyActor`))

(event `self.Sphere.OnComponentBeginOverlap`
  (params (OverlappedComponent :type "PrimitiveComponent Object Reference") (OtherActor :type "Actor Object Reference") (OtherComp :type "PrimitiveComponent Object Reference") (OtherBodyIndex :type Integer) (bFromSweep :type Boolean) (SweepResult :type "HitResult Structure (by ref)"))
  (bind _returnvalue (`self.GetOwner`))
  (if (not (== OtherActor _returnvalue))
    (bind _as0_base (cast `/Game/Blueprints/Characters/Golem/0_Base` OtherActor))
    (`/Game/Blueprints/Characters/Golem/0_Base.Electrocute` _as0_base)
    (`self.K2_DestroyActor`)
    (bind _as0_base_2 (cast `/Game/Blueprints/Characters/Golem/0_Base` _returnvalue)
      (:`then`
        (bind (_playerinfo_playername _playerinfo_rank _playerinfo_items_crafted _playerinfo_products_shipped _playerinfo_tasks_completed _playerinfo_players_knocked_out _playerinfo_players_knocked_out_unarmed _playerinfo_players_knocked_out_1h _playerinfo_players_knocked_out_2h _playerinfo_players_knocked_out_sp _playerinfo_players_knocked_out_ra _playerinfo_times_taunted _playerinfo_pointsround _playerinfo_outfit) (break `/Game/Blueprints/Characters/Golem/Struct_PlayerInfo` (`/Game/Blueprints/Characters/Golem/0_Base.PlayerInfo` _as0_base_2)))
        (set `/Game/Blueprints/Characters/Golem/0_Base.PlayerInfo` (make `/Game/Blueprints/Characters/Golem/Struct_PlayerInfo` _playerinfo_playername _playerinfo_rank _playerinfo_items_crafted _playerinfo_products_shipped _playerinfo_tasks_completed _playerinfo_players_knocked_out _playerinfo_players_knocked_out_unarmed _playerinfo_players_knocked_out_1h _playerinfo_players_knocked_out_2h _playerinfo_players_knocked_out_sp _playerinfo_players_knocked_out_ra _playerinfo_times_taunted (+ _playerinfo_pointsround 10) _playerinfo_outfit) _as0_base_2))
      (:`CastFailed`
        (`self.K2_DestroyActor`)))))

(fn `UserConstructionScript`)