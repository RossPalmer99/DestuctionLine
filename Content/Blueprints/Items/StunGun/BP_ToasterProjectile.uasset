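; BP_ToasterProjectile is a short-lived damaging projectile, filed with the stun gun item.
; Its Sphere overlap ignores the owner, stun guns and itself, then applies damage with the owner as damage causer and destroys the projectile after a brief delay.
; A timed delay from BeginPlay also destroys it after a few seconds.
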(event `self.ReceiveBeginPlay`
  (`KismetSystemLibrary.Delay` 5.0)
  (`self.K2_DestroyActor`))

(event `self.Sphere.OnComponentBeginOverlap`
  (params (OverlappedComponent :type "PrimitiveComponent Object Reference") (OtherActor :type "Actor Object Reference") (OtherComp :type "PrimitiveComponent Object Reference") (OtherBodyIndex :type Integer) (bFromSweep :type Boolean) (SweepResult :type "HitResult Structure (by ref)"))
  (bind _returnvalue (`self.GetOwner`))
  (if (and (!= OtherActor _returnvalue) (!= (`GameplayStatics.GetObjectClass` OtherActor) "/Game/Blueprints/Items/BP_StunGun.BP_StunGun_C") (!= OtherActor self))
    (`GameplayStatics.ApplyDamage` OtherActor 10.0 null _returnvalue)
    (`KismetSystemLibrary.Delay` 0.2)
    (`self.K2_DestroyActor`)))

(fn `UserConstructionScript`)