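; Stack truck item that players pick up to haul colour-matched products or scoop up other players.
; Overlapping products that are not burning snap into three sockets, become fireproof and unload last-in-first-out through Interact.
; When held and empty, it attaches another non-ragdolled player with input disabled, then after a delay detaches and damages them, re-arming its collision later.
; Interact also handles pickup when empty and drop.
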(event `self.DamageDetectCollision.OnComponentBeginOverlap`
  (params (OverlappedComponent :type "PrimitiveComponent Object Reference") (OtherActor :type "Actor Object Reference") (OtherComp :type "PrimitiveComponent Object Reference") (OtherBodyIndex :type Integer) (bFromSweep :type Boolean) (SweepResult :type "HitResult Structure (by ref)"))
  (`|ExecutionSequence`
    (:`then_0`
      (if (not (or (`self.TruckIsCarryingBox`) (`self.TruckIsCarryingPlayer`)))
        (`self.PlayerRef`
          (:`then`
            (bind _as0_base (cast `/Game/Blueprints/Characters/Golem/0_Base` OtherActor))
            (if (and (not (== (`self.PlayerRef`) _as0_base)) (not (`/Game/Blueprints/Characters/Golem/0_Base.InRagdoll` _as0_base)))
              (`self.CollectPlayer` _as0_base)
              (`KismetSystemLibrary.Delay` 5.0)
              (`SceneComponent.K2_DetachFromComponent` (`Actor.RootComponent` _as0_base) "KeepWorld" "KeepRelative" "KeepWorld" true)
              (`GameplayStatics.ApplyDamage` _as0_base 10.0 null self)
              (`PrimitiveComponent.SetCollisionEnabled` (`Character.CapsuleComponent` _as0_base) "QueryAndPhysics")
              (`self.EnableInput` _as0_base (`GameplayStatics.GetPlayerController` (`/Game/Blueprints/Characters/Golem/0_Base.Index` _as0_base)))
              (set `self.TruckIsCarryingPlayer` false)
              (`KismetSystemLibrary.Delay` 7.0)
              (`PrimitiveComponent.SetCollisionEnabled` (`self.DamageDetectCollision`) "QueryAndPhysics")))
          (:`else`))))
    (:`then_1`
      (if (not (`self.TruckIsCarryingPlayer`))
        (bind _asbp_product (cast `/Game/Blueprints/Items/BP_Product` OtherActor))
        (for _array_element (`self.AcceptableColours`)
          (bind (_iteminfo_isproduct _iteminfo_isweapon1h _iteminfo_isweapon2h _iteminfo_isstacktruck _iteminfo_isfireextinguisher _iteminfo_isaccessory _iteminfo_ispowerup _iteminfo_isalarmclock _iteminfo_isbarrel _iteminfo_damage _iteminfo_weaponpower _iteminfo_weaponchip _iteminfo_colour) (break `/Game/Blueprints/Items/Data/Struct_ItemInfo` (`/Game/Blueprints/Items/BP_MasterItem.ItemInfo` _asbp_product)))
          (if (and (not (`/Game/Blueprints/Items/BP_Product.IsOnFire` _asbp_product)) (== _iteminfo_colour _array_element))
            (`self.Stack` _asbp_product)
            (set `/Game/Blueprints/Items/BP_Product.CanBeSetOnFire` false _asbp_product)))))))

(event `/Game/Data/Interact_Interface.Interact`
  (params (Player :type "/Game/Blueprints/Characters/Golem/0_Base Object Reference"))
  (`/Engine/EditorBlueprintResources/StandardMacros.IsValid` (`/Game/Blueprints/Characters/Golem/0_Base.HeldItem` Player)
    (:`Is Valid`
      (message `/Game/Data/Interact_Interface.Drop` self Player self))
    (:`Is Not Valid`
      (`self.PlayerRef`
        (:`then`)
        (:`else`
          (if (`self.TruckIsCarryingBox`)
            (`self.UnstackTruck` Player)
            (else
              (message `/Game/Data/Interact_Interface.PickUp` self Player self))))))))

(fn `CollectPlayer`
  (params (Player :type "/Game/Blueprints/Characters/Golem/0_Base Object Reference"))
  (bind _helditem (`/Game/Blueprints/Characters/Golem/0_Base.HeldItem` Player)
    (:`then`
      (message `/Game/Data/Interact_Interface.Interact` _helditem Player))
    (:`else`
      _))
  (`PrimitiveComponent.SetCollisionEnabled` (`self.DamageDetectCollision`) "NoCollision")
  (`PrimitiveComponent.SetCollisionEnabled` (`Character.CapsuleComponent` Player) "NoCollision")
  (`self.K2_AttachToComponent` Player (`self.StackTruckSM`) "Socket_Golem" "SnapToTarget" "SnapToTarget" "KeepWorld" true)
  (`CharacterMovementComponent.DisableMovement` (`Character.CharacterMovement` Player))
  (`self.DisableInput` Player (`GameplayStatics.GetPlayerController` (`/Game/Blueprints/Characters/Golem/0_Base.Index` Player)))
  (set `self.TruckIsCarryingPlayer` true))

(fn `Stack`
  (params (Item :type "/Game/Blueprints/Items/BP_Product Object Reference"))
  (bind _staticmesh (`/Game/Blueprints/Items/BP_MasterItem.StaticMesh` (`self.CurrentItem`)))
  (bind _staticmesh_2 (`/Game/Blueprints/Items/BP_MasterItem.StaticMesh` (`self.CurrentItem`)))
  (bind _staticmesh_3 (`/Game/Blueprints/Items/BP_MasterItem.StaticMesh` (`self.CurrentItem`)))
  ;[0.5 1 0.5] Check if being carried by player
  (if (== (`self.GetAttachParentActor` Item) null)
    (set `self.TruckIsCarryingBox` true)
    ;[0.5 1 0.5] Put item in position 1
    (if (== (`self.ItemPos`) 0)
      (bind _output_get (set `self.CurrentItem` Item))
      (`self.K2_AttachToComponent` _output_get (`self.StackTruckSM`) "Socket1" "SnapToTarget" "SnapToTarget" "SnapToTarget" true)
      (`PrimitiveComponent.SetSimulatePhysics` _staticmesh_2 false)
      (set `self.ItemPos` 1)
      (`PrimitiveComponent.SetCollisionEnabled` _staticmesh_2 "NoCollision")
      (else
        ;[0.5 1 0.5] Put item in position 2
        (if (== (`self.ItemPos`) 1)
          (bind _output_get_2 (set `self.CurrentItem` Item))
          (`self.K2_AttachToComponent` _output_get_2 (`self.StackTruckSM`) "Socket2" "SnapToTarget" "SnapToTarget" "SnapToTarget" true)
          (`PrimitiveComponent.SetSimulatePhysics` _staticmesh_3 false)
          (set `self.ItemPos` 2)
          (`PrimitiveComponent.SetCollisionEnabled` _staticmesh_3 "NoCollision")
          (else
            ;[0.5 1 0.5] Put item in position 3
            (if (== (`self.ItemPos`) 2)
              (bind _output_get_3 (set `self.CurrentItem` Item))
              (`self.K2_AttachToComponent` _output_get_3 (`self.StackTruckSM`) "Socket3" "SnapToTarget" "SnapToTarget" "SnapToTarget" true)
              (`PrimitiveComponent.SetSimulatePhysics` _staticmesh false)
              (set `self.ItemPos` 3)
              (`PrimitiveComponent.SetCollisionEnabled` _staticmesh "NoCollision"))))))))

(fn `UnstackTruck`
  (params (Player :type "/Game/Blueprints/Characters/Golem/0_Base Object Reference"))
  (bind _currentitem (`self.CurrentItem`))
  (bind _currentitem_2 (`self.CurrentItem`))
  (bind _currentitem_3 (`self.CurrentItem`))
  ;[0.5 1 0.5] Remove first item
  (if (== (`self.ItemPos`) 3)
    (`PrimitiveComponent.SetCollisionEnabled` (`/Game/Blueprints/Items/BP_MasterItem.StaticMesh` _currentitem_2) "QueryAndPhysics")
    (`SceneComponent.K2_DetachFromComponent` (`Actor.RootComponent` _currentitem_2) "KeepWorld" "KeepWorld" "KeepRelative" true)
    (set `/Game/Blueprints/Items/BP_Product.CanBeSetOnFire` true _currentitem_2)
    (message `/Game/Data/Interact_Interface.Interact` _currentitem_2 Player)
    (set `self.ItemPos` 2)
    (for _array_element (`self.GetAttachedActors`)
      (bind _asbp_product (cast `/Game/Blueprints/Items/BP_Product` _array_element))
      (if (== (`self.GetAttachParentSocketName` _array_element) "Socket2")
        (set `self.CurrentItem` _asbp_product)))
    (else
      ;[0.5 1 0.5] Remove second item
      (if (== (`self.ItemPos`) 2)
        (`PrimitiveComponent.SetCollisionEnabled` (`/Game/Blueprints/Items/BP_MasterItem.StaticMesh` _currentitem_3) "QueryAndPhysics")
        (`SceneComponent.K2_DetachFromComponent` (`Actor.RootComponent` _currentitem_3) "KeepWorld" "KeepWorld" "KeepRelative" true)
        (message `/Game/Data/Interact_Interface.Interact` _currentitem_3 Player)
        (set `self.ItemPos` 1)
        (for _array_element_2 (`self.GetAttachedActors`)
          (bind _asbp_product_2 (cast `/Game/Blueprints/Items/BP_Product` _array_element_2))
          (if (== (`self.GetAttachParentSocketName` _array_element_2) "Socket1")
            (set `self.CurrentItem` _asbp_product_2)))
        (else
          ;[0.5 1 0.5] Remove third item
          (if (== (`self.ItemPos`) 1)
            (`PrimitiveComponent.SetCollisionEnabled` (`/Game/Blueprints/Items/BP_MasterItem.StaticMesh` _currentitem) "QueryAndPhysics")
            (`SceneComponent.K2_DetachFromComponent` (`Actor.RootComponent` _currentitem) "KeepWorld" "KeepWorld" "KeepRelative" true)
            (set `/Game/Blueprints/Items/BP_Product.CanBeSetOnFire` true _currentitem)
            (message `/Game/Data/Interact_Interface.Interact` _currentitem Player)
            (set `self.ItemPos` 0)
            (set `self.TruckIsCarryingBox` false)))))))

(fn `UserConstructionScript`
  (`parent.UserConstructionScript`))