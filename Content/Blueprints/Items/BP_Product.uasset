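; Product item box that takes a colour material at BeginPlay, can catch fire and can be thrown.
; Unrecognised product colours become brown boxes without glow, light or widget, with altered collision.
; While burning, it damages overlapping barrels and ignites PlayerRef; after a delay it docks half its point value from that player, or its spawner corner's player, then destroys itself.
; Throwing temporarily records the thrower, but Hit is empty.
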(event `OnFire`
  (bind (_iteminfo_isproduct _iteminfo_isweapon1h _iteminfo_isweapon2h _iteminfo_isstacktruck _iteminfo_isfireextinguisher _iteminfo_isaccessory _iteminfo_ispowerup _iteminfo_isalarmclock _iteminfo_isbarrel _iteminfo_damage _iteminfo_weaponpower _iteminfo_weaponchip _iteminfo_colour _iteminfo_pointvalue) (break `/Game/Blueprints/Items/Data/Struct_ItemInfo` (`self.ItemInfo`)))
  ;[1 1 1] Fire Handling
  (if (`self.CanBeSetOnFire`)
    (set `self.IsOnFire` true)
    (`ActorComponent.Activate` (`self.Fire`) false)
    (`KismetSystemLibrary.Delay` 10.0)
    (bind _playerref (`self.PlayerRef`)
      (:`then`
        (bind (_playerinfo_playername _playerinfo_rank _playerinfo_items_crafted _playerinfo_products_shipped _playerinfo_tasks_completed _playerinfo_players_knocked_out _playerinfo_players_knocked_out_unarmed _playerinfo_players_knocked_out_1h _playerinfo_players_knocked_out_2h _playerinfo_players_knocked_out_sp _playerinfo_players_knocked_out_ra _playerinfo_times_taunted _playerinfo_pointsround _playerinfo_outfit) (break `/Game/Blueprints/Characters/Golem/Struct_PlayerInfo` (`/Game/Blueprints/Characters/Golem/0_Base.PlayerInfo` _playerref)))
        (set `/Game/Blueprints/Characters/Golem/0_Base.PlayerInfo` (make `/Game/Blueprints/Characters/Golem/Struct_PlayerInfo` _playerinfo_playername _playerinfo_rank _playerinfo_items_crafted _playerinfo_products_shipped _playerinfo_tasks_completed _playerinfo_players_knocked_out _playerinfo_players_knocked_out_unarmed _playerinfo_players_knocked_out_1h _playerinfo_players_knocked_out_2h _playerinfo_players_knocked_out_sp _playerinfo_players_knocked_out_ra _playerinfo_times_taunted (- _playerinfo_pointsround (/ _iteminfo_pointvalue 2)) _playerinfo_outfit) _playerref)
        (message `/Game/Data/Interact_Interface.UpdateScore` (`/Game/Blueprints/Characters/Golem/0_Base.Scoreboard` _playerref))
        (`/Game/Blueprints/Characters/Golem/0_Base.Interact With Anything` _playerref))
      (:`else`
        (bind _spawner (`self.Spawner`)
          (:`then`
            (bind _as0_base (cast `/Game/Blueprints/Characters/Golem/0_Base` (`GameplayStatics.GetPlayerCharacter` (`/Game/Blueprints/Environment/BP_ProductSpawner.PlayerCorner` _spawner))))
            (bind (_playerinfo_playername_2 _playerinfo_rank_2 _playerinfo_items_crafted_2 _playerinfo_products_shipped_2 _playerinfo_tasks_completed_2 _playerinfo_players_knocked_out_2 _playerinfo_players_knocked_out_unarmed_2 _playerinfo_players_knocked_out_1h_2 _playerinfo_players_knocked_out_2h_2 _playerinfo_players_knocked_out_sp_2 _playerinfo_players_knocked_out_ra_2 _playerinfo_times_taunted_2 _playerinfo_pointsround_2 _playerinfo_outfit_2) (break `/Game/Blueprints/Characters/Golem/Struct_PlayerInfo` (`/Game/Blueprints/Characters/Golem/0_Base.PlayerInfo` _as0_base)))
            (set `/Game/Blueprints/Characters/Golem/0_Base.PlayerInfo` (make `/Game/Blueprints/Characters/Golem/Struct_PlayerInfo` _playerinfo_playername_2 _playerinfo_rank_2 _playerinfo_items_crafted_2 _playerinfo_products_shipped_2 _playerinfo_tasks_completed_2 _playerinfo_players_knocked_out_2 _playerinfo_players_knocked_out_unarmed_2 _playerinfo_players_knocked_out_1h_2 _playerinfo_players_knocked_out_2h_2 _playerinfo_players_knocked_out_sp_2 _playerinfo_players_knocked_out_ra_2 _playerinfo_times_taunted_2 (- _playerinfo_pointsround_2 (/ _iteminfo_pointvalue 2)) _playerinfo_outfit_2) _as0_base)
            (message `/Game/Data/Interact_Interface.UpdateScore` (`/Game/Blueprints/Characters/Golem/0_Base.Scoreboard` _as0_base)))
          (:`else`))))
    (`self.K2_DestroyActor`)))

(event `self.ReceiveTick`
  (params (DeltaSeconds :type "Float (single-precision)"))
  ;[1 1 1] Fire Handling
  ;;[1 1 1] Damage Handling
  (if (`self.IsOnFire`)
    (for _array_element (`self.GetOverlappingActors` "/Game/Blueprints/DestructibleBlueprints/BP_Barrel.BP_Barrel_C")
      (`GameplayStatics.ApplyDamage` _array_element 10.0 null _array_element))
    (bind _playerref (`self.PlayerRef`)
      (:`then`
        (`/Engine/EditorBlueprintResources/StandardMacros.DoOnce` false
          (:`Completed`
            (`/Game/Blueprints/Characters/Golem/0_Base.OnFire` _playerref true))))
      (:`else`))))

(event `self.Throw`
  (params (PlayerThrowing :type "/Game/Blueprints/Characters/Golem/0_Base Object Reference"))
  ;[1 1 1] Throw
  (set `self.ThrowingPlayer` PlayerThrowing)
  (set `self.HasBeenThrown` true)
  (`KismetSystemLibrary.Delay` 3.0)
  (set `self.HasBeenThrown` false)
  (set `self.ThrowingPlayer` null))

(event `self.ReceiveBeginPlay`
  (bind (_iteminfo_isproduct _iteminfo_isweapon1h _iteminfo_isweapon2h _iteminfo_isstacktruck _iteminfo_isfireextinguisher _iteminfo_isaccessory _iteminfo_ispowerup _iteminfo_isalarmclock _iteminfo_isbarrel _iteminfo_damage _iteminfo_weaponpower _iteminfo_weaponchip _iteminfo_colour) (break `/Game/Blueprints/Items/Data/Struct_ItemInfo` (`self.ItemInfo`)))
  (bind _whileloop_int (`self.WhileLoop Int`))
  ;[1 1 1] Begin Play - sets box colour
  (if _iteminfo_isproduct
    (if (== _iteminfo_colour "Red")
      (`PrimitiveComponent.SetMaterial` (`self.StaticMesh`) 0 "/Game/Materials/Colours/M_red_dark.M_red_dark")
      (elif (== _iteminfo_colour "Green")
        (`PrimitiveComponent.SetMaterial` (`self.StaticMesh`) 0 "/Game/Materials/Colours/M_green.M_green")
        (elif (== _iteminfo_colour "Blue")
          (`PrimitiveComponent.SetMaterial` (`self.StaticMesh`) 0 "/Game/Materials/Colours/M_blue_dark.M_blue_dark")
          (elif (== _iteminfo_colour "Yellow")
            (`PrimitiveComponent.SetMaterial` (`self.StaticMesh`) 0 "/Game/Materials/Colours/M_yellow.M_yellow")
            (elif (== _iteminfo_colour "Grey")
              (`PrimitiveComponent.SetMaterial` (`self.StaticMesh`) 0 "/Game/Materials/Colours/M_grey02.M_grey02")
              (else
                (`PrimitiveComponent.SetMaterial` (`self.StaticMesh`) 0 "/Game/Materials/Colours/M_brown.M_brown")
                (while (< _whileloop_int 5)
                  (`PrimitiveComponent.SetMaterial` (`self.GlowMesh`) _whileloop_int "/Game/Materials/M_invisible.M_invisible")
                  (`LightComponent.SetIntensity` (`self.PointLight`) 0.0)
                  (set `self.WhileLoop Int` (+ (`self.WhileLoop Int`) 1)))
                (`PrimitiveComponent.SetCollisionResponseToAllChannels` (`self.StaticMesh`) "ECR_Block")
                (`ActorComponent.K2_DestroyComponent` (`self.Widget`))
                (`PrimitiveComponent.SetCollisionResponseToChannel` (`self.StaticMesh`) "ECC_Visibility" "ECR_Ignore")))))))))

(event `self.ReceiveHit`
  (params (MyComp :type "PrimitiveComponent Object Reference") (Other :type "Actor Object Reference") (OtherComp :type "PrimitiveComponent Object Reference") (bSelfMoved :type Boolean) (HitLocation :type "Vector Structure") (HitNormal :type "Vector Structure") (NormalImpulse :type "Vector Structure") (Hit :type "HitResult Structure (by ref)"))
  ;[1 1 1] Throw
)

(fn `UserConstructionScript`
  (`parent.UserConstructionScript`))