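; Base Blueprint for physics items that players pick up, drop and swing as weapons, with stubs for throwing.
; Interact toggles pickup and drop, switching physics, pawn collision and socket attachment by item type.
; During an attack, collision overlaps apply multiplier-scaled damage, a launch message and weapon-specific force feedback.
; Helpers award score and KO points, play hit sounds, configure power-up meshes and multipliers, and can turn the item into a hat.
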(event `self.DamageDetectCollision.OnComponentBeginOverlap`
  (params (OverlappedComponent :type "PrimitiveComponent Object Reference") (OtherActor :type "Actor Object Reference") (OtherComp :type "PrimitiveComponent Object Reference") (OtherBodyIndex :type Integer) (bFromSweep :type Boolean) (SweepResult :type "HitResult Structure (by ref)"))
  (bind _playerref (`self.PlayerRef`))
  (bind (_iteminfo_isproduct _iteminfo_isweapon1h _iteminfo_isweapon2h _iteminfo_isstacktruck _iteminfo_isfireextinguisher _iteminfo_isaccessory _iteminfo_ispowerup _iteminfo_isalarmclock _iteminfo_isbarrel _iteminfo_damage) (break `/Game/Blueprints/Items/Data/Struct_ItemInfo` (`self.ItemInfo`)))
  (bind (_iteminfo_isproduct_2 _iteminfo_isweapon1h_2 _iteminfo_isweapon2h_2 _iteminfo_isstacktruck_2 _iteminfo_isfireextinguisher_2 _iteminfo_isaccessory_2 _iteminfo_ispowerup_2 _iteminfo_isalarmclock_2 _iteminfo_isbarrel_2 _iteminfo_damage_2) (break `/Game/Blueprints/Items/Data/Struct_ItemInfo` (`self.ItemInfo`)))
  (bind _playerref_2 (`self.PlayerRef`))
  ;[0.5 1 0.5] ApplyDamage
  (bind _playerref_3 (`self.PlayerRef`)
    (:`then`
      (if (`/Game/Blueprints/Characters/Golem/0_Base.Attack` _playerref_3)
        (`KismetSystemLibrary.Delay` 0.05)
        (`GameplayStatics.ApplyDamage` OtherActor (* _iteminfo_damage (`/Game/Blueprints/Characters/Golem/0_Base.DamageMultiplier` (`self.PlayerRef`))) null self)
        (message `/Game/Data/Interact_Interface.Launch` OtherActor true self)
        (if _iteminfo_isweapon1h_2
          (`PlayerController.K2_ClientPlayForceFeedback` (`GameplayStatics.GetPlayerController` (`/Game/Blueprints/Characters/Golem/0_Base.Index` _playerref_2)) (`/Game/Blueprints/Characters/Golem/0_Base.FF_1hHit` _playerref_2) "None" false false false)
          (elif _iteminfo_isweapon2h_2
            (`PlayerController.K2_ClientPlayForceFeedback` (`GameplayStatics.GetPlayerController` (`/Game/Blueprints/Characters/Golem/0_Base.Index` _playerref)) (`/Game/Blueprints/Characters/Golem/0_Base.FF_2hHit` _playerref) "None" false false false)))))
    (:`else`)))

(event `/Game/Data/Interact_Interface.Interact`
  (params (Player :type "/Game/Blueprints/Characters/Golem/0_Base Object Reference"))
  (bind _helditem (`/Game/Blueprints/Characters/Golem/0_Base.HeldItem` Player))
  ;[0.5 1 0.5] InteractHandler
  (`/Engine/EditorBlueprintResources/StandardMacros.IsValid` _helditem
    (:`Is Valid`
      (if (== _helditem self)
        (message `/Game/Data/Interact_Interface.Drop` self Player self)
        (else
          (message `/Game/Data/Interact_Interface.Drop` _helditem Player _helditem))))
    (:`Is Not Valid`
      (set `self.HasBeenThrown` false)
      (`self.PlayerRef`
        (:`then`)
        (:`else`
          (message `/Game/Data/Interact_Interface.PickUp` self Player self))))))

(event `/Game/Data/Interact_Interface.KOPoints`
  ;[0.5 1 0.5] Points
  (bind _playerref (`self.PlayerRef`)
    (:`then`
      (`/Game/Blueprints/Characters/Golem/0_Base.CheckKOStat` _playerref _playerref)
      (`/Game/Blueprints/Characters/Golem/0_Base.AddKOPoints` _playerref)
      (message `/Game/Data/Interact_Interface.UpdateScore` (`/Game/Blueprints/Characters/Golem/0_Base.Scoreboard` _playerref)))
    (:`else`)))

(event `/Game/Data/Interact_Interface.Points`
  (bind (_iteminfo_isproduct _iteminfo_isweapon1h _iteminfo_isweapon2h _iteminfo_isstacktruck _iteminfo_isfireextinguisher _iteminfo_isaccessory _iteminfo_ispowerup _iteminfo_isalarmclock _iteminfo_isbarrel _iteminfo_damage) (break `/Game/Blueprints/Items/Data/Struct_ItemInfo` (`self.ItemInfo`)))
  ;[0.5 1 0.5] Points
  (bind _playerref (`self.PlayerRef`)
    (:`then`
      (`self.GivePoints` _iteminfo_damage _playerref)
      (message `/Game/Data/Interact_Interface.UpdateScore` (`/Game/Blueprints/Characters/Golem/0_Base.Scoreboard` _playerref))
      (`self.PlaySound`))
    (:`else`)))

(event `/Game/Data/Interact_Interface.PickUp`
  (params (Player :type "/Game/Blueprints/Characters/Golem/0_Base Object Reference") (Item :type "/Game/Blueprints/Items/BP_MasterItem Object Reference"))
  (bind _staticmesh (`/Game/Blueprints/Items/BP_MasterItem.StaticMesh` Item))
  (bind _playerref (`self.PlayerRef`))
  (bind (_iteminfo_isproduct _iteminfo_isweapon1h _iteminfo_isweapon2h _iteminfo_isstacktruck _iteminfo_isfireextinguisher _iteminfo_isaccessory _iteminfo_ispowerup _iteminfo_isalarmclock _iteminfo_isbarrel _iteminfo_damage _iteminfo_weaponpower _iteminfo_weaponchip _iteminfo_colour _iteminfo_pointvalue _iteminfo_isstungun) (break `/Game/Blueprints/Items/Data/Struct_ItemInfo` (`self.ItemInfo`)))
  ;[0.5 1 0.5] Pick Me Up
  (bind _output_get (set `self.PlayerRef` Player))
  (`PrimitiveComponent.SetCollisionResponseToChannel` _staticmesh "ECC_Pawn" "ECR_Overlap")
  (`PrimitiveComponent.SetSimulatePhysics` _staticmesh false)
  (`KismetSystemLibrary.Delay` 1e-06)
  (if _iteminfo_isbarrel
    (bind _mesh (`Character.Mesh` _output_get))
    (`self.K2_AttachToComponent` Item _mesh "BarrelGrip" "SnapToTarget" "SnapToTarget" "KeepWorld" true)
    (elif _iteminfo_isstungun
      (if (== _iteminfo_colour "Toast")
        (`self.K2_AttachToComponent` Item _mesh "ToasterGrip" "SnapToTarget" "SnapToTarget" "KeepWorld" true)
        (else
          (`self.K2_AttachToComponent` Item _mesh "Grip" "SnapToTarget" "SnapToTarget" "KeepWorld" true :!label _label)))
      (else
        (goto _label))))
  (`SceneComponent.SetVisibility` (`self.GlowMesh`) false false)
  (`SceneComponent.SetVisibility` (`self.Widget`) false false)
  (`SceneComponent.SetVisibility` (`self.PointLight`) false false)
  (message `/Game/Data/Interact_Interface.PickUp` _playerref _playerref self)
  (`PlayerController.K2_ClientPlayForceFeedback` (`GameplayStatics.GetPlayerController` (`/Game/Blueprints/Characters/Golem/0_Base.Index` _playerref)) (`/Game/Blueprints/Characters/Golem/0_Base.FF_Hit` _playerref) "None" false false false))

(event `/Game/Data/Interact_Interface.Drop`
  (params (Player :type "/Game/Blueprints/Characters/Golem/0_Base Object Reference") (Item :type "/Game/Blueprints/Items/BP_MasterItem Object Reference"))
  (bind _staticmesh (`self.StaticMesh`))
  ;[0.5 1 0.5] Drop Me
  (message `/Game/Data/Interact_Interface.Drop` Player Player Item)
  (`SceneComponent.K2_DetachFromComponent` (`self.RootComponent`) "KeepWorld" "KeepWorld" "KeepWorld" true)
  (set `self.PlayerRef` null)
  (`PrimitiveComponent.SetCollisionResponseToChannel` _staticmesh "ECC_Pawn" "ECR_Block")
  (`PrimitiveComponent.SetSimulatePhysics` _staticmesh true)
  (`SceneComponent.SetVisibility` (`self.GlowMesh`) false false)
  (`SceneComponent.SetVisibility` (`self.Widget`) false false)
  (`SceneComponent.SetVisibility` (`self.PointLight`) false false)
  (`self.ResetDoOnce`))

(event `LoseHat`
  ;[1 1 1] Drop Hat
)

(event `ResetDoOnce`
  ;[0.5 1 0.5] Drop Me
)

(event `Throw`
  (params (PlayerThrowing :type "/Game/Blueprints/Characters/Golem/0_Base Object Reference"))
  ;[0.5 1 0.5] Drop Me
)

(event `self.ReceiveBeginPlay`
  ;[0.5 1 0.5] Begin Play
  (`SceneComponent.SetAbsolute` (`self.Sphere`) false true false)
  (`PrimitiveComponent.SetSimulatePhysics` (`self.StaticMesh`) true))

(fn `GivePlayerHat`
  (params (IsAccessory :type Boolean) (Player :type "/Game/Blueprints/Characters/Golem/0_Base Object Reference") (`Player's Skeletal Mesh` :type "SkeletalMeshComponent Object Reference"))
  (bind _staticmesh (`self.StaticMesh`))
  (if IsAccessory
    (bind _output_get (set `self.HatOwner` Player))
    (if (< (`/Game/Blueprints/Characters/Golem/0_Base.Health` _output_get) 1)
      (if (> (`KismetMathLibrary.RandomInteger` 5) 4)
        (`/Game/Blueprints/Characters/Golem/0_Base.Interact With Anything` (`self.PlayerRef`))
        (bind _output_get_2 (set `/Game/Blueprints/Characters/Golem/0_Base.NewHat` self (`self.HatOwner`)))
        (`self.K2_AttachToComponent` _output_get_2 `Player's Skeletal Mesh` "ConeSocket" "SnapToTarget" "SnapToTarget" "KeepRelative" true)
        (`PrimitiveComponent.SetSimulatePhysics` _staticmesh false)
        (`PrimitiveComponent.SetCollisionResponseToChannel` _staticmesh "ECC_Visibility" "ECR_Ignore")))))

(fn `GivePoints`
  (params (Points :type Integer) (Player :type "/Game/Blueprints/Characters/Golem/0_Base Object Reference"))
  (bind (_playerinfo_playername _playerinfo_rank _playerinfo_items_crafted _playerinfo_products_shipped _playerinfo_tasks_completed _playerinfo_players_knocked_out _playerinfo_players_knocked_out_unarmed _playerinfo_players_knocked_out_1h _playerinfo_players_knocked_out_2h _playerinfo_players_knocked_out_sp _playerinfo_players_knocked_out_ra _playerinfo_times_taunted _playerinfo_pointsround _playerinfo_outfit) (break `/Game/Blueprints/Characters/Golem/Struct_PlayerInfo` (`/Game/Blueprints/Characters/Golem/0_Base.PlayerInfo` Player)))
  (set `/Game/Blueprints/Characters/Golem/0_Base.PlayerInfo` (make `/Game/Blueprints/Characters/Golem/Struct_PlayerInfo` _playerinfo_playername _playerinfo_rank _playerinfo_items_crafted _playerinfo_products_shipped _playerinfo_tasks_completed _playerinfo_players_knocked_out _playerinfo_players_knocked_out_unarmed _playerinfo_players_knocked_out_1h _playerinfo_players_knocked_out_2h _playerinfo_players_knocked_out_sp _playerinfo_players_knocked_out_ra _playerinfo_times_taunted (+ _playerinfo_pointsround (`KismetMathLibrary.FTrunc` (* Points (`/Game/Blueprints/Characters/Golem/0_Base.PointMultiplier` Player)))) _playerinfo_outfit) Player))

(fn `PlaySound`
  (if (`|EnumEquality` (`self.SoundInfo`) "NewEnumerator0")
    (`GameplayStatics.SpawnSoundAttached` "/Game/Audio/SFX/SE_MetalHitMetal_Cue.SE_MetalHitMetal_Cue" (`self.StaticMesh`) "None" (0.0 0.0 0.0) (struct) "KeepRelativeOffset" true 0.33 1.0 0.0 null null)
    (elif (`|EnumEquality` (`self.SoundInfo`) "NewEnumerator1")
      (`GameplayStatics.SpawnSoundAttached` "/Game/Audio/SFX/SE_BaseballBatHit.SE_BaseballBatHit" (`self.StaticMesh`) "None" (0.0 0.0 0.0) (struct) "KeepRelativeOffset" true 0.33 1.0 0.0 null null))))

(fn `SetPowerUP_Damage`
  (params (IsPositive :type Boolean))
  (bind (_powerinfo_power _powerinfo_ispowerup _powerinfo_pointmultiplier _powerinfo_speedmultiplier _powerinfo_damagemultiplier _powerinfo_candjump) (break `/Game/Blueprints/Items/Data/Struct_PowerInfo` (`self.PowerInfo`)))
  (bind _glowmesh (`self.GlowMesh`))
  (bind _staticmesh (`self.StaticMesh`))
  (bind (_powerinfo_power_2 _powerinfo_ispowerup_2 _powerinfo_pointmultiplier_2 _powerinfo_speedmultiplier_2 _powerinfo_damagemultiplier_2 _powerinfo_candjump_2) (break `/Game/Blueprints/Items/Data/Struct_PowerInfo` (`self.PowerInfo`)))
  (if IsPositive
    (set `self.PowerInfo` (make `/Game/Blueprints/Items/Data/Struct_PowerInfo` _powerinfo_power _powerinfo_ispowerup _powerinfo_pointmultiplier _powerinfo_speedmultiplier 2.0 _powerinfo_candjump))
    (`StaticMeshComponent.SetStaticMesh` _staticmesh "/Game/Assets/Shared/PowerUPs/MoreAssets_model_increased_damage_item.MoreAssets_model_increased_damage_item")
    (`StaticMeshComponent.SetStaticMesh` _glowmesh "/Game/Assets/Shared/PowerUPs/MoreAssets_model_increased_damage_item.MoreAssets_model_increased_damage_item")
    (else
      (set `self.PowerInfo` (make `/Game/Blueprints/Items/Data/Struct_PowerInfo` _powerinfo_power_2 _powerinfo_ispowerup_2 _powerinfo_pointmultiplier_2 _powerinfo_speedmultiplier_2 0.5 _powerinfo_candjump_2))
      (`StaticMeshComponent.SetStaticMesh` _staticmesh "/Game/Assets/Shared/PowerUPs/MoreAssets_model_decreased_damage_item.MoreAssets_model_decreased_damage_item")
      (`StaticMeshComponent.SetStaticMesh` _glowmesh "/Game/Assets/Shared/PowerUPs/MoreAssets_model_decreased_damage_item.MoreAssets_model_decreased_damage_item"))))

(fn `SetPowerUP_Jump`
  (params (CanDJump :type Boolean))
  (bind _glowmesh (`self.GlowMesh`))
  (bind _staticmesh (`self.StaticMesh`))
  (if CanDJump
    (`StaticMeshComponent.SetStaticMesh` _staticmesh "/Game/Assets/Shared/PowerUPs/MoreAssets_model_increased_jump_item_orange.MoreAssets_model_increased_jump_item_orange")
    (`StaticMeshComponent.SetStaticMesh` _glowmesh "/Game/Assets/Shared/PowerUPs/MoreAssets_model_increased_jump_item_orange.MoreAssets_model_increased_jump_item_orange")
    (else
      (`StaticMeshComponent.SetStaticMesh` _staticmesh "/Game/Assets/Shared/PowerUPs/MoreAssets_model_decreased_jump_item_brown.MoreAssets_model_decreased_jump_item_brown")
      (`StaticMeshComponent.SetStaticMesh` _glowmesh "/Game/Assets/Shared/PowerUPs/MoreAssets_model_decreased_jump_item_brown.MoreAssets_model_decreased_jump_item_brown"))))

(fn `SetPowerUP_Points`
  (params (IsPositive :type Boolean))
  (bind (_powerinfo_power _powerinfo_ispowerup _powerinfo_pointmultiplier _powerinfo_speedmultiplier _powerinfo_damagemultiplier _powerinfo_candjump) (break `/Game/Blueprints/Items/Data/Struct_PowerInfo` (`self.PowerInfo`)))
  (bind _glowmesh (`self.GlowMesh`))
  (bind _staticmesh (`self.StaticMesh`))
  (bind (_powerinfo_power_2 _powerinfo_ispowerup_2 _powerinfo_pointmultiplier_2 _powerinfo_speedmultiplier_2 _powerinfo_damagemultiplier_2 _powerinfo_candjump_2) (break `/Game/Blueprints/Items/Data/Struct_PowerInfo` (`self.PowerInfo`)))
  (if IsPositive
    (set `self.PowerInfo` (make `/Game/Blueprints/Items/Data/Struct_PowerInfo` _powerinfo_power _powerinfo_ispowerup 1.5 _powerinfo_speedmultiplier _powerinfo_damagemultiplier _powerinfo_candjump))
    (`StaticMeshComponent.SetStaticMesh` _staticmesh "/Game/Assets/Shared/PowerUPs/MoreAssets_model_increased_points_stopwatch.MoreAssets_model_increased_points_stopwatch")
    (`StaticMeshComponent.SetStaticMesh` _glowmesh "/Game/Assets/Shared/PowerUPs/MoreAssets_model_increased_points_stopwatch.MoreAssets_model_increased_points_stopwatch")
    (else
      (set `self.PowerInfo` (make `/Game/Blueprints/Items/Data/Struct_PowerInfo` _powerinfo_power_2 _powerinfo_ispowerup_2 0.5 _powerinfo_speedmultiplier_2 _powerinfo_damagemultiplier_2 _powerinfo_candjump_2))
      (`StaticMeshComponent.SetStaticMesh` _staticmesh "/Game/Assets/Shared/PowerUPs/MoreAssets_model_decreased_points_stopwatch.MoreAssets_model_decreased_points_stopwatch")
      (`StaticMeshComponent.SetStaticMesh` _glowmesh "/Game/Assets/Shared/PowerUPs/MoreAssets_model_decreased_points_stopwatch.MoreAssets_model_decreased_points_stopwatch"))))

(fn `SetPowerUP_Speed`
  (params (IsPositive :type Boolean))
  (bind (_powerinfo_power _powerinfo_ispowerup _powerinfo_pointmultiplier _powerinfo_speedmultiplier _powerinfo_damagemultiplier _powerinfo_candjump) (break `/Game/Blueprints/Items/Data/Struct_PowerInfo` (`self.PowerInfo`)))
  (bind _glowmesh (`self.GlowMesh`))
  (bind _staticmesh (`self.StaticMesh`))
  (bind (_powerinfo_power_2 _powerinfo_ispowerup_2 _powerinfo_pointmultiplier_2 _powerinfo_speedmultiplier_2 _powerinfo_damagemultiplier_2 _powerinfo_candjump_2) (break `/Game/Blueprints/Items/Data/Struct_PowerInfo` (`self.PowerInfo`)))
  (if IsPositive
    (set `self.PowerInfo` (make `/Game/Blueprints/Items/Data/Struct_PowerInfo` _powerinfo_power _powerinfo_ispowerup _powerinfo_pointmultiplier 1.5 _powerinfo_damagemultiplier _powerinfo_candjump))
    (`StaticMeshComponent.SetStaticMesh` _staticmesh "/Game/Assets/Shared/PowerUPs/MoreAssets_model_increased_speed_item.MoreAssets_model_increased_speed_item")
    (`StaticMeshComponent.SetStaticMesh` _glowmesh "/Game/Assets/Shared/PowerUPs/MoreAssets_model_increased_speed_item.MoreAssets_model_increased_speed_item")
    (else
      (set `self.PowerInfo` (make `/Game/Blueprints/Items/Data/Struct_PowerInfo` _powerinfo_power_2 _powerinfo_ispowerup_2 _powerinfo_pointmultiplier_2 0.8 _powerinfo_damagemultiplier_2 _powerinfo_candjump_2))
      (`StaticMeshComponent.SetStaticMesh` _staticmesh "/Game/Assets/Shared/PowerUPs/MoreAssets_model_decreased_speed_item.MoreAssets_model_decreased_speed_item")
      (`StaticMeshComponent.SetStaticMesh` _glowmesh "/Game/Assets/Shared/PowerUPs/MoreAssets_model_decreased_speed_item.MoreAssets_model_decreased_speed_item"))))

(fn `UserConstructionScript`)