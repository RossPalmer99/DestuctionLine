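; BP_StunGun is a stun gun item with a rare toaster variant.
; On BeginPlay, after the parent logic, a random roll between MinimumRandVal and 100 that lands on 100 sets the ItemInfo colour to "Toast".
; If the item is flagged as a stun gun, that colour swaps both the static and glow meshes to a toaster model.
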(event `self.ReceiveBeginPlay`
  (bind (_iteminfo_isproduct _iteminfo_isweapon1h _iteminfo_isweapon2h _iteminfo_isstacktruck _iteminfo_isfireextinguisher _iteminfo_isaccessory _iteminfo_ispowerup _iteminfo_isalarmclock _iteminfo_isbarrel _iteminfo_damage _iteminfo_weaponpower _iteminfo_weaponchip _iteminfo_colour _iteminfo_pointvalue _iteminfo_isstungun) (break `/Game/Blueprints/Items/Data/Struct_ItemInfo` (`self.ItemInfo`)))
  (bind (_iteminfo_isproduct_2 _iteminfo_isweapon1h_2 _iteminfo_isweapon2h_2 _iteminfo_isstacktruck_2 _iteminfo_isfireextinguisher_2 _iteminfo_isaccessory_2 _iteminfo_ispowerup_2 _iteminfo_isalarmclock_2 _iteminfo_isbarrel_2 _iteminfo_damage_2 _iteminfo_weaponpower_2 _iteminfo_weaponchip_2 _iteminfo_colour_2 _iteminfo_pointvalue_2 _iteminfo_isstungun_2) (break `/Game/Blueprints/Items/Data/Struct_ItemInfo` (`self.ItemInfo`)))
  (`parent.ReceiveBeginPlay`)
  (if (== (`KismetMathLibrary.RandomIntegerInRange` (`self.MinimumRandVal`) 100) 100)
    (set `self.ItemInfo` (make `/Game/Blueprints/Items/Data/Struct_ItemInfo` _iteminfo_isproduct_2 _iteminfo_isweapon1h_2 _iteminfo_isweapon2h_2 _iteminfo_isstacktruck_2 _iteminfo_isfireextinguisher_2 _iteminfo_isaccessory_2 _iteminfo_ispowerup_2 _iteminfo_isalarmclock_2 _iteminfo_isbarrel_2 _iteminfo_damage_2 _iteminfo_weaponpower_2 _iteminfo_weaponchip_2 "Toast" _iteminfo_pointvalue_2 _iteminfo_isstungun_2))
    (if _iteminfo_isstungun
      (if (== _iteminfo_colour "Toast")
        (`StaticMeshComponent.SetStaticMesh` (`self.StaticMesh`) "/Game/Assets/Break_Room/Decoration/MoreAssets_model_toaster.MoreAssets_model_toaster")
        (`StaticMeshComponent.SetStaticMesh` (`self.GlowMesh`) "/Game/Assets/Break_Room/Decoration/MoreAssets_model_toaster.MoreAssets_model_toaster")))))

(fn `UserConstructionScript`
  (`parent.UserConstructionScript`))