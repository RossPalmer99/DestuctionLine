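; Game mode that spawns local players and runs an optional timed round ending on a scoreboard.
; At BeginPlay it creates players, spawns a 0_Base pawn at the PlayerStart tagged with each index, possesses it and assigns a name.
; A one-second Delay on Tick drives the minute/second countdown.
; At zero it collects every pawn's PlayerInfo, briefly shows WBP_ScoreBoard, then opens map_breakroom; the HUD creation is unconnected.
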(event `self.ReceiveBeginPlay`
  (`self.GetPlayerStartPoints`)
  (`self.SpawnPlayers`))

(event `self.ReceiveTick`
  (params (DeltaSeconds :type "Float (single-precision)"))
  (`KismetSystemLibrary.Delay` 1.0)
  (if (`self.GamemodeIsTimed`)
    (`|ExecutionSequence`
      (:`then_0`
        (if (`self.GameRunning`)
          (set `self.Time_Sec` (- (`self.Time_Sec`) 1))
          (if (< (`self.Time_Sec`) 0)
            (set `self.Time_Min` (- (`self.Time_Min`) 1))
            (set `self.Time_Sec` 59))))
      (:`then_1`
        (if (and (== (`self.Time_Sec`) 0) (== (`self.Time_Min`) 0))
          (bind _outactors (`GameplayStatics.GetAllActorsOfClass` "/Game/Blueprints/Characters/Golem/0_Base.0_Base_C"))
          (for _array_element _outactors
            (`KismetArrayLibrary.Array_Add` (`self.PlayerInfoArray`) (`/Game/Blueprints/Characters/Golem/0_Base.PlayerInfo` _array_element)))
          (set `self.GameRunning` false)
          (`/Engine/EditorBlueprintResources/StandardMacros.DoOnce` false
            (:`Completed`
              (bind _returnvalue (`|CreateWidget` "/Game/Blueprints/Characters/WBPs/ScoreBoard/WBP_ScoreBoard.WBP_ScoreBoard_C"))
              (set `/Game/Blueprints/Characters/WBPs/ScoreBoard/WBP_ScoreBoard.IsAllowedToUpdate` false _returnvalue)
              (`UserWidget.AddToViewport` _returnvalue 0)
              (`KismetSystemLibrary.Delay` 10.0)
              (`Widget.RemoveFromParent` _returnvalue)
              (`GameplayStatics.OpenLevel` "map_breakroom"))))))))

(fn `GetPlayerStartPoints`
  (bind _outactors (`GameplayStatics.GetAllActorsOfClass` "/Script/Engine.PlayerStart"))
  (set `self.PlayerStartArray` _outactors))

(fn `SpawnPlayers`
  (bind _index (`self.Index`))
  (for _index_2 (range (`self.MaxPlayerCount`))
    (set `self.Index` _index_2)
    (for _array_element (`self.PlayerStartArray`)
      (if (== (`PlayerStart.PlayerStartTag` _array_element) (`KismetStringLibrary.Conv_StringToName` (`KismetStringLibrary.Conv_IntToString` (`self.Index`))))
        (`GameplayStatics.CreatePlayer` _index)
        (bind _returnvalue (`|SpawnActorFromClass` "/Game/Blueprints/Characters/Golem/0_Base.0_Base_C" (`self.GetTransform` _array_element) "AlwaysSpawn" "OverrideRootScale" null (struct) 100 null))
        (`Controller.Possess` (`GameplayStatics.GetPlayerController` _index) _returnvalue)
        (bind _output_get (set `/Game/Blueprints/Characters/Golem/0_Base.Index` _index _returnvalue))
        (bind (_playerinfo_playername _playerinfo_rank _playerinfo_items_crafted _playerinfo_products_shipped _playerinfo_tasks_completed _playerinfo_players_knocked_out _playerinfo_players_knocked_out_unarmed _playerinfo_players_knocked_out_1h _playerinfo_players_knocked_out_2h _playerinfo_players_knocked_out_sp _playerinfo_players_knocked_out_ra _playerinfo_times_taunted _playerinfo_pointsround _playerinfo_outfit) (break `/Game/Blueprints/Characters/Golem/Struct_PlayerInfo` (`/Game/Blueprints/Characters/Golem/0_Base.PlayerInfo` _returnvalue)))
        (set `/Game/Blueprints/Characters/Golem/0_Base.PlayerInfo` (make `/Game/Blueprints/Characters/Golem/Struct_PlayerInfo` (`|GetArrayItem` (`self.Names`) _output_get) _playerinfo_rank _playerinfo_items_crafted _playerinfo_products_shipped _playerinfo_tasks_completed _playerinfo_players_knocked_out _playerinfo_players_knocked_out_unarmed _playerinfo_players_knocked_out_1h _playerinfo_players_knocked_out_2h _playerinfo_players_knocked_out_sp _playerinfo_players_knocked_out_ra _playerinfo_times_taunted _playerinfo_pointsround _playerinfo_outfit) _returnvalue)
        (`KismetArrayLibrary.Array_AddUnique` (`self.Players`) _returnvalue)))))

(fn `UserConstructionScript`)