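; BP_PlayerController is the player controller that opens the pause and exit menu widgets.
; The PauseGame input creates UI_PauseMenu, stores it, and switches to UI-only input focused on it, without calling SetGamePaused.
; It shows the cursor only when the pressing key is not a gamepad key.
; An ExitMenu event opens UI_ExitMenu the same way, with the cursor hidden.
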(event `/Game/Data/Interact_Interface.ExitMenu`
  (params (Index :type Integer) (ExitDoor :type "/Game/Blueprints/Environment/BP_ExitDoor Object Reference"))
  (bind _returnvalue (`|CreateWidget` "/Game/UI/UMG/Main_Menu/UI_ExitMenu.UI_ExitMenu_C"))
  (bind _output_get (set `self.ExitMenuRef` _returnvalue))
  (`UserWidget.AddToViewport` _output_get 0)
  (`WidgetBlueprintLibrary.SetInputMode_UIOnlyEx` self (`self.ExitMenuRef`))
  (set `self.bShowMouseCursor` false))

(event `InputAction|PauseGame`
  (params (Key :type "Key Structure"))
  (:`Pressed`
    (if (`KismetInputLibrary.Key_IsGamepadKey` Key)
      (bind _returnvalue (`|CreateWidget` "/Game/UI/UMG/Main_Menu/UI_PauseMenu.UI_PauseMenu_C"))
      (bind _output_get (set `self.PauseMenu` _returnvalue))
      (`UserWidget.AddToViewport` _output_get 0)
      (`WidgetBlueprintLibrary.SetInputMode_UIOnlyEx` self (`self.PauseMenu`))
      (set `self.bShowMouseCursor` false)
      (else
        (bind _returnvalue_2 (`|CreateWidget` "/Game/UI/UMG/Main_Menu/UI_PauseMenu.UI_PauseMenu_C"))
        (bind _output_get_2 (set `self.PauseMenu` _returnvalue_2))
        (`UserWidget.AddToViewport` _output_get_2 0)
        (`WidgetBlueprintLibrary.SetInputMode_UIOnlyEx` self (`self.PauseMenu`))
        (set `self.bShowMouseCursor` true)))))

(fn `UserConstructionScript`)