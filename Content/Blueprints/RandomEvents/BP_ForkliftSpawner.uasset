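; Random event actor that periodically sends an existing BP_Forklift along its spline in a randomly chosen direction.
; A looping timer, with its interval randomized once at BeginPlay, hides and moves every forklift to a spline end, keeping the last as the driven one.
; A twice-played alarm precedes the reveal, then a timeline drives it along the spline, played in reverse with yaw flipped for the opposite direction.
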(event `self.ReceiveBeginPlay`
  (`KismetSystemLibrary.K2_SetTimerDelegate` (delegate `ForkliftMoving`) (`KismetMathLibrary.RandomFloatInRange` (`self.MinTime`) (`self.MaxTime`)) true))

(event `ForkliftMoving`
  (bind _output_get (set `self.RightSpawn` (`KismetMathLibrary.RandomBool`)))
  (if _output_get
    (`self.SpawnForkliftRight`)
    (set `self.IsTriggered` true)
    (`|ExecutionSequence`
      (:`then_0`
        _)
      (:`then_1`
        (`KismetSystemLibrary.Delay` 1.718)))
    (bind _returnvalue (`GameplayStatics.SpawnSoundAttached` "/Game/Audio/SFX/SE_Alarm.SE_Alarm" (`self.DefaultSceneRoot`) "None" (0.0 0.0 0.0) (struct) "KeepRelativeOffset" false 0.5 1.0 0.0 null null))
    (set `self.Alarm` _returnvalue)
    (`KismetSystemLibrary.Delay` 2.0)
    (`self.SetActorHiddenInGame` (`self.Forklift`) false)
    (bind (_direction _traveldistance) (`Timeline|ForkliftDrivesLeft` :!via `PlayFromStart`)
      (:`Update`
        (bind _returnvalue_2 (* _traveldistance (`SplineComponent.GetSplineLength` (`self.Spline`))))
        (`SceneComponent.K2_SetWorldLocation` (`Actor.RootComponent` (`self.Forklift`)) (`SplineComponent.GetLocationAtDistanceAlongSpline` (`self.Spline`) _returnvalue_2 "World") false false)
        (`SceneComponent.K2_SetRelativeRotation` (`Actor.RootComponent` (`self.Forklift`)) (`SplineComponent.GetRotationAtDistanceAlongSpline` (`self.Spline`) _returnvalue_2 "Local") false false))
      (:`Finished`
        (set `self.IsTriggered` false)
        (`KismetSystemLibrary.Delay` 1.0)))
    (else
      (`self.SpawnForkliftLeft`)
      (set `self.IsTriggered` true)
      (`|ExecutionSequence`
        (:`then_0`
          _)
        (:`then_1`
          (`KismetSystemLibrary.Delay` 1.718)))
      (bind _returnvalue_3 (`GameplayStatics.SpawnSoundAttached` "/Game/Audio/SFX/SE_Alarm.SE_Alarm" (`self.DefaultSceneRoot`) "None" (0.0 0.0 0.0) (struct) "KeepRelativeOffset" false 0.5 1.0 0.0 null null))
      (set `self.Alarm` _returnvalue_3)
      (`KismetSystemLibrary.Delay` 2.0)
      (`self.SetActorHiddenInGame` (`self.Forklift`) false)
      (bind (_direction_2 _traveldistance_2) (`Timeline|ForkliftDrivesRight` :!via `ReverseFromEnd`)
        (:`Update`
          (bind _returnvalue_4 (* _traveldistance_2 (`SplineComponent.GetSplineLength` (`self.Spline`))))
          (`SceneComponent.K2_SetWorldLocation` (`Actor.RootComponent` (`self.Forklift`)) (`SplineComponent.GetLocationAtDistanceAlongSpline` (`self.Spline`) _returnvalue_4 "World") false false)
          (bind (_returnvalue_roll _returnvalue_pitch _returnvalue_yaw) (`KismetMathLibrary.BreakRotator` (`SplineComponent.GetRotationAtDistanceAlongSpline` (`self.Spline`) _returnvalue_4 "Local")))
          (`SceneComponent.K2_SetRelativeRotation` (`Actor.RootComponent` (`self.Forklift`)) (`KismetMathLibrary.MakeRotator` _returnvalue_roll _returnvalue_pitch (- _returnvalue_yaw 180.0)) false false))
        (:`Finished`
          (set `self.IsTriggered` false)
          (`KismetSystemLibrary.Delay` 1.0))))))

(fn `SpawnForkliftLeft`
  (bind _returnvalue (`SplineComponent.GetSplineLength` (`self.Spline`)))
  (bind (_returnvalue_location _returnvalue_rotation) (`KismetMathLibrary.BreakTransform` (`KismetMathLibrary.MakeTransform` (`SplineComponent.GetLocationAtDistanceAlongSpline` (`self.Spline`) _returnvalue "World") (`SplineComponent.GetRotationAtDistanceAlongSpline` (`self.Spline`) _returnvalue "World"))))
  (bind _outactors (`GameplayStatics.GetAllActorsOfClass` "/Game/Blueprints/RandomEvents/BP_Forklift.BP_Forklift_C"))
  (for _array_element _outactors
    (bind _output_get (set `self.Forklift` _array_element))
    (`self.SetActorHiddenInGame` _output_get true)
    (`self.K2_SetActorLocationAndRotation` _output_get _returnvalue_location _returnvalue_rotation false false)))

(fn `SpawnForkliftRight`
  (bind _returnvalue (`SplineComponent.GetSplineLength` (`self.Spline`)))
  (bind _returnvalue_2 (- _returnvalue _returnvalue))
  (bind (_returnvalue_location _returnvalue_rotation) (`KismetMathLibrary.BreakTransform` (`KismetMathLibrary.MakeTransform` (`SplineComponent.GetLocationAtDistanceAlongSpline` (`self.Spline`) _returnvalue_2 "World") (`SplineComponent.GetRotationAtDistanceAlongSpline` (`self.Spline`) _returnvalue_2 "World"))))
  (bind _outactors (`GameplayStatics.GetAllActorsOfClass` "/Game/Blueprints/RandomEvents/BP_Forklift.BP_Forklift_C"))
  (for _array_element _outactors
    (bind _output_get (set `self.Forklift` _array_element))
    (`self.SetActorHiddenInGame` _output_get true)
    (`self.K2_SetActorLocationAndRotation` _output_get _returnvalue_location _returnvalue_rotation false false)))

(fn `UserConstructionScript`)