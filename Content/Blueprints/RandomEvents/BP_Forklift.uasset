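; Forklift hazard, filed under random events, that damages and launches actors it touches.
; Tick continuously spins a sphere component and rolls the four wheels by RollerSpeed, with no movement of the forklift itself in this graph.
; Overlaps on the front, back, side and fork collision volumes call KnockOutPlayer, which filters that volume's overlapping actors by AttackableComponents, then applies damage, force feedback and a LaunchMessage to each.
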(event `self.ReceiveTick`
  (params (DeltaSeconds :type "Float (single-precision)"))
  (`SceneComponent.K2_AddRelativeRotation` (`self.Sphere`) (`KismetMathLibrary.MakeRotator` 0.0 0.0 (* DeltaSeconds 360.0)) false false)
  (`SceneComponent.K2_AddRelativeRotation` (`self.FLWheel`) (`KismetMathLibrary.MakeRotator` (`self.RollerSpeed`)) false false)
  (`SceneComponent.K2_AddRelativeRotation` (`self.FRWheel`) (`KismetMathLibrary.MakeRotator` (`self.RollerSpeed`)) false false)
  (`SceneComponent.K2_AddRelativeRotation` (`self.BLWheel`) (`KismetMathLibrary.MakeRotator` (`self.RollerSpeed`)) false false)
  (`SceneComponent.K2_AddRelativeRotation` (`self.BRWheel`) (`KismetMathLibrary.MakeRotator` (`self.RollerSpeed`)) false false))

(event `self.Collision_front.OnComponentBeginOverlap`
  (params (OverlappedComponent :type "PrimitiveComponent Object Reference") (OtherActor :type "Actor Object Reference") (OtherComp :type "PrimitiveComponent Object Reference") (OtherBodyIndex :type Integer) (bFromSweep :type Boolean) (SweepResult :type "HitResult Structure (by ref)"))
  (`self.Knock out player` (`self.Collision_front`)))

(event `self.Collision_back.OnComponentBeginOverlap`
  (params (OverlappedComponent :type "PrimitiveComponent Object Reference") (OtherActor :type "Actor Object Reference") (OtherComp :type "PrimitiveComponent Object Reference") (OtherBodyIndex :type Integer) (bFromSweep :type Boolean) (SweepResult :type "HitResult Structure (by ref)"))
  (`self.Knock out player` (`self.Collision_back`)))

(event `self.Collision_left.OnComponentBeginOverlap`
  (params (OverlappedComponent :type "PrimitiveComponent Object Reference") (OtherActor :type "Actor Object Reference") (OtherComp :type "PrimitiveComponent Object Reference") (OtherBodyIndex :type Integer) (bFromSweep :type Boolean) (SweepResult :type "HitResult Structure (by ref)"))
  (`self.Knock out player` (`self.Collision_left`)))

(event `self.Collision_right.OnComponentBeginOverlap`
  (params (OverlappedComponent :type "PrimitiveComponent Object Reference") (OtherActor :type "Actor Object Reference") (OtherComp :type "PrimitiveComponent Object Reference") (OtherBodyIndex :type Integer) (bFromSweep :type Boolean) (SweepResult :type "HitResult Structure (by ref)"))
  (`self.Knock out player` (`self.Collision_right`)))

(event `self.Collision_forks.OnComponentBeginOverlap`
  (params (OverlappedComponent :type "PrimitiveComponent Object Reference") (OtherActor :type "Actor Object Reference") (OtherComp :type "PrimitiveComponent Object Reference") (OtherBodyIndex :type Integer) (bFromSweep :type Boolean) (SweepResult :type "HitResult Structure (by ref)"))
  (`self.Knock out player` (`self.Collision_forks`)))

(fn `Knock out player`
  (params (Collision :type "BoxComponent Object Reference"))
  (for _array_element (`self.AttackableComponents`)
    (for _array_element_2 (`PrimitiveComponent.GetOverlappingActors` Collision _array_element)
      (`GameplayStatics.ApplyDamage` _array_element_2 20.0 null self)
      (`GameplayStatics.SpawnForceFeedbackAttached` "/Game/Blueprints/Characters/Golem/Vibration_Pack/FF_FLT.FF_FLT" (`self.Forklift`) "None" (0.0 0.0 0.0) (struct) "SnapToTarget" false false 1.0 0.0 null)
      (message `/Game/Data/Interact_Interface.Launch` _array_element_2 true null))))

(fn `UserConstructionScript`)