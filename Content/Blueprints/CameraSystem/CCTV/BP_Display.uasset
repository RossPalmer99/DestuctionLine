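; BP_Display is a CCTV monitor display with four screens and a periodic scoreboard overlay.
; AssignCamera uses the camera's ID to pick a quadrant, giving it a dynamic instance of that screen's monitor material fed by the supplied texture.
; Tick runs a ten-second Delay into a FlipFlop, alternately creating and destroying the scoreboard widget component and toggling its background.
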(event `/Game/Data/Interact_Interface.AssignCamera`
  (params (ScreenTexture :type "TextureRenderTarget2D Object Reference") (CCTV :type "/Game/Blueprints/CameraSystem/CCTV/BP_CCTV Object Reference"))
  (bind _id (`/Game/Blueprints/CameraSystem/CCTV/BP_CCTV.ID` CCTV))
  (set `self.Texture` ScreenTexture)
  (if (== _id 0)
    (bind _returnvalue (`PrimitiveComponent.CreateDynamicMaterialInstance` (`self.TL`) 0 "/Game/Blueprints/CameraSystem/CCTV/M_Monitor_Normal.M_Monitor_Normal" "None"))
    (bind _output_get (set `self.MIDTVScreen` _returnvalue))
    (`MaterialInstanceDynamic.SetTextureParameterValue` _output_get "ScreenTexture01" (`self.Texture`))
    (elif (== _id 1)
      (bind _returnvalue_2 (`PrimitiveComponent.CreateDynamicMaterialInstance` (`self.TR`) 0 "/Game/Blueprints/CameraSystem/CCTV/M_Monitor_FastScan.M_Monitor_FastScan" "None"))
      (bind _output_get_2 (set `self.MIDTVScreen` _returnvalue_2))
      (`MaterialInstanceDynamic.SetTextureParameterValue` _output_get_2 "ScreenTexture01" (`self.Texture`))
      (elif (== _id 2)
        (bind _returnvalue_3 (`PrimitiveComponent.CreateDynamicMaterialInstance` (`self.BL`) 0 "/Game/Blueprints/CameraSystem/CCTV/M_Monitor_Alt.M_Monitor_Alt" "None"))
        (bind _output_get_3 (set `self.MIDTVScreen` _returnvalue_3))
        (`MaterialInstanceDynamic.SetTextureParameterValue` _output_get_3 "ScreenTexture01" (`self.Texture`))
        (elif (== _id 3)
          (bind _returnvalue_4 (`PrimitiveComponent.CreateDynamicMaterialInstance` (`self.BR`) 0 "/Game/Blueprints/CameraSystem/CCTV/M_Monitor_SlowScan.M_Monitor_SlowScan" "None"))
          (bind _output_get_4 (set `self.MIDTVScreen` _returnvalue_4))
          (`MaterialInstanceDynamic.SetTextureParameterValue` _output_get_4 "ScreenTexture01" (`self.Texture`)))))))

(event `self.ReceiveBeginPlay`)

(event `self.ReceiveTick`
  (params (DeltaSeconds :type "Float (single-precision)"))
  (`KismetSystemLibrary.Delay` 10.0)
  (`/Engine/EditorBlueprintResources/StandardMacros.FlipFlop`
    (:`A`
      (bind _returnvalue (`AddComponent|NODE_AddWidgetComponent-0`))
      (bind _output_get (set `self.Scoreboard` _returnvalue))
      (`SceneComponent.K2_AddRelativeLocation` _output_get (0.0 10.0 -120.0) false true)
      (`SceneComponent.K2_AddWorldRotation` _output_get (struct :`Yaw` 90.0) false false)
      (`SceneComponent.SetVisibility` (`self.Scoreboard Background`) true false))
    (:`B`
      (`ActorComponent.K2_DestroyComponent` (`self.Scoreboard`))
      (`SceneComponent.SetVisibility` (`self.Scoreboard Background`) false false))))

(fn `UserConstructionScript`)