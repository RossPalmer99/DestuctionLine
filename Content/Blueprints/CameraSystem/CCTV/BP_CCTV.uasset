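; CCTV camera that sweeps back and forth, tracks targets it spots, and feeds its view to a coupled monitor.
; With a valid monitor, it creates a render target and captures the scene on a timer at a set framerate, not every frame.
; A repeating pawn sphere trace finds camera-target interface actors, switching timelines from sweep to look-at follow.
; When the target is lost, it eases back and resumes sweeping.
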(event `SetFramerate`
  (bind _cameracapture (`self.CameraCapture`))
  (if true
    (`KismetSystemLibrary.K2_SetTimerDelegate` (delegate `CameraUpdate`) (/ 1.0 (`self.Framerate`)) true)
    (set `SceneCaptureComponent.bCaptureEveryFrame` false _cameracapture)
    (set `SceneCaptureComponent.bCaptureOnMovement` false _cameracapture)))

(event `CameraUpdate`
  (`SceneCaptureComponent2D.CaptureScene` (`self.CameraCapture`)))

(event `self.ReceiveBeginPlay`
  (`self.CoupledMonitor`
    (:`then`
      (bind _returnvalue (`CanvasRenderTarget2D.CreateCanvasRenderTarget2D` "/Script/Engine.CanvasRenderTarget2D" 1920 1080))
      (bind _output_get (set `SceneCaptureComponent2D.TextureTarget` _returnvalue (`self.CameraCapture`)))
      (message `/Game/Data/Interact_Interface.AssignCamera` (`self.CoupledMonitor`) _output_get self)
      (`self.SetFramerate`)
      (`KismetSystemLibrary.K2_SetTimerDelegate` (delegate `LookForPlayer`) 0.1 true)
      (bind (_direction _newtrack_0) (`Timeline|CameraSweep_Timeline` :!via `PlayFromStart` :!label _label)
        (:`Update`
          (`SceneComponent.K2_SetRelativeRotation` (`self.Camera`) (`KismetMathLibrary.MakeRotator` 0.0 -20.0 (`KismetMathLibrary.Lerp` 0.0 40.0 _newtrack_0)) false false))))
    (:`else`)))

(event `LookForPlayer`
  (bind _scene (`self.Scene`))
  (bind _returnvalue (`SceneComponent.K2_GetComponentLocation` _scene))
  (bind _outhit (`KismetSystemLibrary.SphereTraceSingleForObjects` _returnvalue (+ _returnvalue (* (`SceneComponent.GetForwardVector` _scene) 1000.0)) 200.0 (`|MakeArray` "ObjectTypeQuery3" :!type "EObjectTypeQuery Enum")))
  (bind (_bblockinghit _binitialoverlap _time _distance _location _impactpoint _normal _impactnormal _physmat _hitactor) (`GameplayStatics.BreakHitResult` _outhit))
  (if (`KismetSystemLibrary.DoesImplementInterface` _hitactor "/Game/Blueprints/CameraSystem/CCTV/BPInterface_CameraTarget.BPInterface_CameraTarget_C")
    (`|ExecutionSequence`
      (:`then_0`
        (goto _label_4 :!via `Reset`))
      (:`then_1`
        (bind (_direction _newtrack_0) (`Timeline|ReturnToSweep_Timeline` :!via `Stop` :!label _label_2)
          (:`Update`
            (`SceneComponent.K2_SetRelativeRotation` (`self.Camera`) (`KismetMathLibrary.RLerp` (stale _output_get) (struct :`Pitch` -20.0) _newtrack_0) false false))
          (:`Finished`
            (goto _label :!via `PlayFromStart`))))
      (:`then_2`
        (goto _label :!via `Stop`))
      (:`then_3`
        (set `self.Player` _hitactor)
        (`Timeline|FollowPlayer_Timeline` :!via `PlayFromStart` :!label _label_3
          (:`Update`
            (bind _looktarget (message `/Game/Blueprints/CameraSystem/CCTV/BPInterface_CameraTarget.GetLookTarget` (`self.Player`)))
            (`SceneComponent.K2_SetWorldRotation` (`self.Camera`) (`KismetMathLibrary.FindLookAtRotation` (`SceneComponent.K2_GetComponentLocation` (`self.Camera`)) _looktarget) false false)))))
    (else
      (`|ExecutionSequence`
        (:`then_0`
          (goto _label_3 :!via `Stop`))
        (:`then_1`
          (`/Engine/EditorBlueprintResources/StandardMacros.DoOnce` false :!label _label_4
            (:`Completed`
              (bind _output_get (set `self.LastSeenLocation` (`SceneComponent.RelativeRotation` (`self.Camera`))))
              (goto _label_2 :!via `PlayFromStart`))))))))

(fn `UserConstructionScript`)